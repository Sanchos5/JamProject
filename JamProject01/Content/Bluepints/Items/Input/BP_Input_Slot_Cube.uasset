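; Input slot actor for cubes that identifies which tagged actor enters its trigger volume.
; On overlap, a Sequence checks tags BP1 through BP4, each gated by its own InIndexCube flag, then prints a debug message and stores the matching number in IndexRaw.
; The logic looks unfinished: most helper functions are stubs, and IndexSumReq increments a counter but is not called in this graph.
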(event OnComponentBeginOverlap(TriggerVolume)
  (params (OverlappedComponent :type Primitive%20Component%20Object%20Reference) (OtherActor :type Actor%20Object%20Reference) (OtherComp :type Primitive%20Component%20Object%20Reference) (OtherBodyIndex :type Integer) (bFromSweep :type Boolean) (SweepResult :type Hit%20Result%20Structure%20%28by%20ref%29))
  ;[1 1 1] Я в душе не ебу как это реализовать
  (Utilities|FlowControl|Sequence
    (:then_0
      (if (and (Actor|ActorHasTag OtherActor "BP1") (Variables|Default|GetInIndexCube))
        (Development|PrintString "Да Has Tag BP1")
        (Variables|Default|SetIndexRaw 1)))
    (:then_1
      (if (and (Actor|ActorHasTag OtherActor "BP2") (Variables|Default|GetInIndexCube2))
        (Development|PrintString "Да Has Tag BP2")
        (Variables|Default|SetIndexRaw 2)))
    (:then_2
      (if (and (Actor|ActorHasTag OtherActor "BP3") (Variables|Default|GetInIndexCube3))
        (Development|PrintString "Да Has Tag BP3")
        (Variables|Default|SetIndexRaw 3)))
    (:then_3
      (if (and (Actor|ActorHasTag OtherActor "BP4") (Variables|Default|GetInIndexCube4))
        (Development|PrintString "Да Has Tag BP4")
        (Variables|Default|SetIndexRaw 4)))))

(event EventBeginPlay
  (|CallParentFunction))

(event Collision|EventActorBeginOverlap
  (params (OtherActor :type Actor%20Object%20Reference))
  (|CallParentFunction OtherActor))

(event EventTick
  (params (DeltaSeconds :type Float%20%28single-precision%29))
  (|CallParentFunction DeltaSeconds) ; This node is disabled and will not be called.\nDrag off pins to build functionality.
)

(fn ConstructionScript
  (|CallParentFunction))

(fn CheckIndex)

(fn GetDropItemIndex
  (return 0))

(fn GetPickupItem
  (return false))

(fn IndexSumReq
  (Variables|Default|SetIdexSumReqCurrent (+ (Variables|Default|GetIdexSumReqCurrent) 1)))

(fn FunctionTestovaya
  (return false false false false))