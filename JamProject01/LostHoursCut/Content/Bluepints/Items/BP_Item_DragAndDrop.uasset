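; BP_Item_DragAndDrop is an item Blueprint that, by its name and getters, represents a drag-and-drop item for pickup and dropping.
; It answers item queries through small functions: GetPickupItem always returns true, GetDropItemIndex returns IndexItem, and GetItemType returns a fixed enum entry.
; GetMesh returns no value.
; BeginPlay and construction only call the parent, and an unconnected Mesh collision-response node never runs.
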(event EventBeginPlay
  (|CallParentFunction))

(event Collision|EventActorBeginOverlap
  (params (OtherActor :type Actor%20Object%20Reference)))

(event EventTick
  (params (DeltaSeconds :type Float%20%28single-precision%29)))

(fn ConstructionScript
  (|CallParentFunction))

(fn GetPickupItem
  (return true))

(fn GetDropItemIndex
  (return (Variables|Default|GetIndexItem)))

(fn GetMesh
  (return 0))

(fn GetItemType
  (return "NewEnumerator0"))