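; Rotatable pyramid piece for the second puzzle, solved when three pieces share the same yaw.
; Interacting plays a sound and a timeline that turns the mesh a quarter turn, with a DoOnce blocking re-triggers until it finishes.
; Each timeline update gathers the yaw of every BP_PiramidaDown and compares the first three within a tolerance.
; A match calls Puzzle2Success on BP_ThirdPersonGameMode, once per piece instance.
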(event Custom|CustomEvent
  (bind _piramidpiecesyaw (Variables|Default|GetPiramidPiecesYaw))
  (bind _output (Utilities|Array|Get(acopy) _piramidpiecesyaw 2))
  (bind _output_2 (Utilities|Array|Get(acopy) _piramidpiecesyaw 1))
  (bind _output_3 (Utilities|Array|Get(acopy) _piramidpiecesyaw))
  (bind _returnvalue (Math|Conversions|ToFloat(Integer) _output_3))
  (bind _returnvalue_2 (Math|Conversions|ToFloat(Integer) _output_2))
  (bind _returnvalue_3 (Math|Conversions|ToFloat(Integer) _output))
  (Utilities|FlowControl|DoOnce false) ; enters at Reset
)

(event EventBeginPlay
  (|CallParentFunction) ; This node is disabled and will not be called.\nDrag off pins to build functionality.
)

(event Collision|EventActorBeginOverlap
  (params (OtherActor :type Actor%20Object%20Reference)))

(event EventTick
  (params (DeltaSeconds :type Float%20%28single-precision%29)))

(event EventInteractwith
  (bind _piramidpiecesyaw (Variables|Default|GetPiramidPiecesYaw))
  (bind _output (Utilities|Array|Get(acopy) _piramidpiecesyaw 2))
  (bind _output_2 (Utilities|Array|Get(acopy) _piramidpiecesyaw 1))
  (bind _output_3 (Utilities|Array|Get(acopy) _piramidpiecesyaw))
  (bind _returnvalue (Math|Conversions|ToFloat(Integer) _output_3))
  (bind _returnvalue_2 (Math|Conversions|ToFloat(Integer) _output_2))
  (bind _returnvalue_3 (Math|Conversions|ToFloat(Integer) _output))
  (Utilities|FlowControl|DoOnce false
    (:Completed
      (Audio|PlaySound2D "/Game/Bluepints/Items/SFX/SmallSoundKit/SSKWav/ClothesWav/Shirt_NRM_01.Shirt_NRM_01" 1.5 0.05 0.0 0 0)
      (bind _rotation (Timeline|Timeline PlayFromStart)
        (:Update
          (bind _output_get (Variables|Default|SetSetRotator (Math|Rotator|Lerp(Rotator) (Variables|Default|GetSetRotator) (Math|Rotator|MakeRotator 0.0 0.0 (+ (Variables|Default|GetNewRotation) -9e+01)) _rotation)))
          (Transformation|SetWorldRotation (Variables|Default|GetStaticMesh) _output_get false false)
          ;[1 1 1] после каждого вращения предмета класса пирамидка > проверить yaw всех остальных частей пирамидки
          (bind _outactors (Actor|GetAllActorsOfClass "BP_PiramidaDown_C"))
          (for (_array_element _array_index) _outactors
            (Utilities|Array|SetArrayElem (Variables|Default|GetPiramidPiecesYaw) _array_index (Math|Float|Truncate (.yaw (Transformation|GetWorldRotation (Variables|BP_PiramidaDown_C|GetStaticMesh _array_element))))))
          (if (Math|Boolean|ANDBoolean (Math|Float|NearlyEqual(Float) _returnvalue _returnvalue_2 5.0) (Math|Float|NearlyEqual(Float) _returnvalue _returnvalue_3 5.0) (Math|Float|NearlyEqual(Float) _returnvalue_2 _returnvalue_3 5.0))
            (Utilities|FlowControl|DoOnce false
              (:Completed
                (bind _asbp_third_person_game_mode (Utilities|Casting|CastToBP_ThirdPersonGameMode (Game|GetGameMode)))
                (Default|Puzzle2Success _asbp_third_person_game_mode)))))
        (:Finished
          (CallFunction|CustomEvent)
          (Variables|Default|SetNewRotation (+ (Variables|Default|GetNewRotation) -9e+01)))))))

(fn ConstructionScript
  (|CallParentFunction))

(fn GetPickupItem
  (return false))