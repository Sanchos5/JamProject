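; Stage light actor with a trigger box that advances the game mode's path puzzle when the player enters.
; LightN selects the trigger's role: start the path, or run the step matching PuzzlePathN, each once after delays.
; The last step calls CurtainCall, swings the tagged finale door open through Tick interpolation and shows the finale widget.
; Events switch the RectLight on with sound, off, or fade it dramatically using a looping timer.
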(event OnComponentBeginOverlap(Box)
  (params (OverlappedComponent :type Primitive%20Component%20Object%20Reference) (OtherActor :type Actor%20Object%20Reference) (OtherComp :type Primitive%20Component%20Object%20Reference) (OtherBodyIndex :type Integer) (bFromSweep :type Boolean) (SweepResult :type Hit%20Result%20Structure%20%28by%20ref%29))
  (if (== OtherActor (Game|Player|GetPlayerPawn 0))
    (switch int (Variables|Default|GetLightN)
      (:0
        (switch int (Variables|/Game/Bluepints/BP_ThirdPersonGameMode.BP_ThirdPersonGameMode_C|GetPuzzlePathN (Variables|Default|GetGamemodeRef))
          (:1
            (Utilities|FlowControl|DoOnce false
              (:Completed
                (Utilities|FlowControl|Delay 2.0)
                (Default|PathPuzzle1 (Variables|Default|GetGamemodeRef)))))
          (:2
            (Utilities|FlowControl|DoOnce false
              (:Completed
                (Utilities|FlowControl|Delay 4.0)
                (Default|PathPuzzle2 (Variables|Default|GetGamemodeRef)))))
          (:3
            (Utilities|FlowControl|DoOnce false
              (:Completed
                (Utilities|FlowControl|Delay 4.0)
                (Default|PathPuzzle3 (Variables|Default|GetGamemodeRef)))))
          (:4
            (Utilities|FlowControl|DoOnce false
              (:Completed
                (Default|CurtainCall (Variables|Default|GetGamemodeRef))
                (Utilities|FlowControl|Delay 1e+01)
                (Variables|Default|SetbFinaleDoor true)
                (Audio|PlaySound2D "/Game/Bluepints/Items/SFX/SmallSoundKit/SSKWav/DoorsWav/Drs_Wood_Door_Open_01.Drs_Wood_Door_Open_01" 0.8 0.9 0.0 0 0)
                (Utilities|FlowControl|Delay 4.0)
                (bind _returnvalue (UserInterface|CreateWidget "/Game/UI/Widgets/WBP_Finale.WBP_Finale_C" (Game|GetPlayerController 0)))
                (UserInterface|Viewport|AddtoViewport _returnvalue 0)
                (Widget|SetVisibility _returnvalue "Visible"))))))
      (:1
        (Utilities|FlowControl|DoOnce false
          (:Completed
            ;[1 1 1] playerstart part zero
            (Utilities|FlowControl|Delay 1.5)
            (Default|PathZero (Variables|Default|GetGamemodeRef))))))))

(event Custom|LightON
  ;[1 1 1] home
  (Audio|PlaySound2D "/Game/Music/LightSound.LightSound" 0.5 1.0 0.0 0 0)
  (Rendering|SetVisibility (Variables|Default|GetRectLight) true false))

(event Custom|LightOFF
  ;[1 1 1] home
  (Rendering|SetVisibility (Variables|Default|GetRectLight) false false))

(event Custom|DramaticLightOff
  ;[1 1 1] DramaticLightOff
  (switch int (Variables|Default|GetLightN)
    (:Default
      _)
    (:0
      (Utilities|FlowControl|Delay 3.0)))
  (bind _returnvalue (Utilities|Time|SetTimerbyEvent (delegate Custom|FadeOut) 0.05 true)))

(event Custom|FadeOut
  (bind _rectlight (Variables|Default|GetRectLight))
  (bind _intensity (Variables|/Script/Engine.LightComponentBase|GetIntensity _rectlight))
  ;[1 1 1] DramaticLightOff
  (if (> _intensity 0.0)
    (Rendering|Components|Light|SetIntensity _rectlight (- _intensity 1e+02))
    (else
      (Utilities|Time|InvalidateTimerHandle (stale Custom|DramaticLightOff _returnvalue)))))

(event EventBeginPlay
  (bind _asbp_third_person_game_mode (Utilities|Casting|CastToBP_ThirdPersonGameMode (Game|GetGameMode)))
  (Variables|Default|SetGamemodeRef _asbp_third_person_game_mode))

(event Collision|EventActorBeginOverlap
  (params (OtherActor :type Actor%20Object%20Reference)))

(event EventTick
  (params (DeltaSeconds :type Float%20%28single-precision%29))
  ;[1 1 1] FinaleDoor
  (Utilities|FlowControl|Sequence
    (:then_0
      (if (Variables|Default|GetbFinaleDoor)
        (Transformation|SetActorRotation (stale _output_get) (Class|KismetMathLibrary|RInterptoConstant (Transformation|GetActorRotation (stale _output_get)) "0.000000,180.000000,0.000000" DeltaSeconds 2e+01))
        (else
          (Utilities|FlowControl|DoOnce false
            (:Completed
              (bind _outactors (Actor|GetAllActorswithTag "FinaleDoor"))
              (bind _output_get (Variables|Default|SetDoor (Utilities|Array|Get(acopy) _outactors))))))))))

(fn ConstructionScript)