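; BP_StolInteract is an interactable, apparently a table, that moves the player into a fixed view; its Interactwith event is empty.
; SwitchCamera saves the player transform, disables movement, gravity and capsule collision, then timeline-lerps the player to an Arrow once.
; FirstSwitchCamera restores walk speed and lerps the camera back toward the saved transform, leaving gravity and collision unrestored.
; Disconnected logic would make BP_Item_DragAndDrop meshes block Visibility traces.
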(event Custom|FirstSwitchCamera
  (bind _as_bp_player (Variables|Default|GetAs%20BP%20Player))
  (bind _followcamera (Variables|/Game/Bluepints/Core/Player/BP_FPS_Character.BP_FPS_Character_C|GetFollowCamera _as_bp_player))
  (Variables|/Script/Engine.CameraComponent|SetbUsePawnControlRotation _followcamera true)
  (Variables|/Game/Bluepints/Core/Player/BP_FPS_Character.BP_FPS_Character_C|SetIsLook? _as_bp_player true)
  (Variables|/Script/Engine.CharacterMovementComponent|SetMaxWalkSpeed (Variables|/Script/Engine.Character|GetCharacterMovement _as_bp_player) 3e+02)
  (bind _newtrack_0 (Timeline|Timeline_0 PlayFromStart)
    (:Update
      (Transformation|SetWorldTransform _followcamera (Math|Transform|Lerp(Transform) (Transformation|GetWorldTransform (Variables|Default|GetArrow)) (Variables|Default|GetSetTransformCamera) _newtrack_0) false false))))

(event Custom|SwitchCamera
  (bind _as_bp_player (Variables|Default|GetAs%20BP%20Player))
  (bind _charactermovement (Variables|/Script/Engine.Character|GetCharacterMovement _as_bp_player))
  (Utilities|FlowControl|DoOnce false
    (:Completed
      (Variables|/Script/Engine.SpringArmComponent|SetbUsePawnControlRotation (Variables|/Game/Bluepints/Core/Player/BP_FPS_Character.BP_FPS_Character_C|GetSpringArm _as_bp_player) false)
      (Variables|Default|SetSetTransformCamera (Transformation|GetActorTransform _as_bp_player))
      (Variables|/Game/Bluepints/Core/Player/BP_FPS_Character.BP_FPS_Character_C|SetIsLook? _as_bp_player true)
      (Variables|/Script/Engine.CharacterMovementComponent|SetMaxWalkSpeed _charactermovement 0.0)
      (Variables|/Script/Engine.CharacterMovementComponent|SetGravityScale _charactermovement 0.0)
      (Collision|SetCollisionEnabled (Variables|/Script/Engine.Character|GetCapsuleComponent _as_bp_player) "NoCollision")
      (bind _newtrack_0 (Timeline|Timeline PlayFromStart)
        (:Update
          (Transformation|SetActorTransform _as_bp_player (Math|Transform|Lerp(Transform) (Variables|Default|GetSetTransformCamera) (Transformation|GetWorldTransform (Variables|Default|GetArrow)) _newtrack_0)))))))

(event EventBeginPlay
  (|CallParentFunction)
  (Variables|Default|SetAs%20BP%20Player (CallFunction|FindPlayerCast)))

(event Collision|EventActorBeginOverlap
  (params (OtherActor :type Actor%20Object%20Reference)))

(event EventTick
  (params (DeltaSeconds :type Float%20%28single-precision%29)))

(event EventInteractwith)

(fn ConstructionScript
  (|CallParentFunction))

(fn GetPickupItem
  (return false))