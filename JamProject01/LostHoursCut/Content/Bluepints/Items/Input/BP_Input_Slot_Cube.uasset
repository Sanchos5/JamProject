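; BP_Input_Slot_Cube is a slot for the first puzzle, which completes when four slots hold mannequins.
; Overlap with a BP_Item_DragAndDrop flags the slot as filled and, once per slot, plays a concrete sound and counts filled slots across all instances.
; A count of four calls Puzzle1Success on BP_ThirdPersonGameMode.
; The filled flag is never cleared, as no end-overlap handling exists.
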(event EventBeginPlay
  (|CallParentFunction)
  (Variables|Default|SetMannequinInPla 0))

(event Collision|EventActorBeginOverlap
  (params (OtherActor :type Actor%20Object%20Reference))
  (|CallParentFunction OtherActor)
  (if (== (Utilities|GetClass OtherActor) "/Game/Bluepints/Items/BP_Item_DragAndDrop.BP_Item_DragAndDrop_C")
    (Variables|Default|SetMannequinInPlace true)
    (Utilities|FlowControl|DoOnce false
      (:Completed
        (Audio|PlaySound2D "/Game/Bluepints/Items/SFX/SmallSoundKit/SSKWav/FootstepsWav/S_Concrete_Mono_1.S_Concrete_Mono_1" 0.2 1.0 0.0 0 0)
        (bind _outactors (Actor|GetAllActorsOfClass "BP_Input_Slot_Cube_C"))
        (for _array_element _outactors
          (if (Variables|BP_Input_Slot_Cube_C|GetMannequinInPlace _array_element)
            (bind _result (Math|Integer|IncrementInt (Variables|Default|GetMannequinInPla)))))
        (if (== (Variables|Default|GetMannequinInPla) 4)
          ;[1 1 1] success
          (bind _asbp_third_person_game_mode (Utilities|Casting|CastToBP_ThirdPersonGameMode (Game|GetGameMode)))
          (Default|Puzzle1Success _asbp_third_person_game_mode))))))

(event EventTick
  (params (DeltaSeconds :type Float%20%28single-precision%29))
  (|CallParentFunction DeltaSeconds) ; This node is disabled and will not be called.\nDrag off pins to build functionality.
)

(fn ConstructionScript
  (|CallParentFunction))