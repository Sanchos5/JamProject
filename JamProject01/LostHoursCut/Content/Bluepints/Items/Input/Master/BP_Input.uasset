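; BP_Input is a master Blueprint for input items that switch connected objects on and off.
; Set State On and Set State Off store a boolean State, then loop through Connections calling On or Off on each.
; Construction and Update Children are empty, while the item queries for type, mesh, fracture, drop index and pickup return only defaults.
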(fn ConstructionScript)

(fn UpdateChildren)

(fn SetStateon
  (Variables|Runtime|SetState true)
  (for _array_element (Variables|Data|GetConnections)
    (Default|On _array_element)))

(fn SetStateOff
  (Variables|Runtime|SetState false)
  (for _array_element (Variables|Data|GetConnections)
    (Default|Off _array_element)))

(fn GetFractureBool
  (return false))

(fn GetItemType
  (return "NewEnumerator0"))

(fn GetMesh
  (return 0))

(fn GetDropItemIndex
  (return 0))

(fn GetPickupItem
  (return false))