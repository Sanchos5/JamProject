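; BP_Note is an interactable note item that opens a note screen when the player interacts with it.
; Interactwith creates a new WBP_Note widget and adds it to the viewport, passing it no data and keeping no check for an existing one.
; BeginPlay, the CustomDepth toggle and the construction script only forward to the parent class.
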(event EventBeginPlay
  (|CallParentFunction))

(event Collision|EventActorBeginOverlap
  (params (OtherActor :type Actor%20Object%20Reference))
  (|CallParentFunction OtherActor) ; This node is disabled and will not be called.\nDrag off pins to build functionality.
)

(event EventTick
  (params (DeltaSeconds :type Float%20%28single-precision%29))
  (|CallParentFunction DeltaSeconds) ; This node is disabled and will not be called.\nDrag off pins to build functionality.
)

(event EventInteractwith
  (bind _returnvalue (UserInterface|CreateWidget "/Game/UI/WBP_Note.WBP_Note_C"))
  (UserInterface|Viewport|AddtoViewport _returnvalue 0))

(event EventCustomDepth
  (params (IsCustomDepth :type Boolean))
  (|CallParentFunction IsCustomDepth))

(fn ConstructionScript
  (|CallParentFunction))