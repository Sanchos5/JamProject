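; BP_Wind is a level wind volume that pushes the player along its Arrow's forward direction and changes their walk speed while inside.
; Overlap toggles a state that Tick reads to interpolate MaxWalkSpeed toward the set value or back to the speed saved on entry.
; The push moves the player's root component each tick without sweep.
; A desert ambience fades in on entry and out on exit, then is destroyed after a delay.
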(event Custom|WIND
  (bind _playerref (Variables|Default|GetPlayerRef))
  (bind _rootcomponent (Variables|/Script/Engine.Actor|GetRootComponent _playerref))
  (bind _returnvalue (Transformation|GetWorldLocation _rootcomponent))
  (Transformation|SetWorldLocation _rootcomponent (Math|Interpolation|VInterptoConstant _returnvalue (+ _returnvalue (* (Math|Vector|GetForwardVector (Variables|Default|GetArrow)) 9)) (stale EventTick DeltaSeconds) 4e+01) false false))

(event Collision|EventActorBeginOverlap
  (params (OtherActor :type Actor%20Object%20Reference))
  (if (== OtherActor (Game|Player|GetPlayerPawn 0))
    (bind _asthird_person_character (Utilities|Casting|CastToThirdPersonCharacter OtherActor))
    (Variables|Default|SetMaxSpeedReset (Variables|/Script/Engine.CharacterMovementComponent|GetMaxWalkSpeed (Variables|/Script/Engine.Character|GetCharacterMovement _asthird_person_character)))
    (Variables|Default|SetPlayerRef _asthird_person_character)
    (Variables|Default|SetSetSpeed 1)
    (bind _returnvalue (Audio|SpawnSound2D "/Game/SmallSoundKit/SSKWav/AmbienceWav/Amb_Desert_01.Amb_Desert_01" 1.0 1.0 0.0 0 false false))
    (bind _output_get (Variables|Default|SetSFX _returnvalue))
    (Audio|Components|Audio|FadeIn _output_get 0.2 0.6 0.0 "Linear" :!class /Script/Engine.AudioComponent)
    (Development|PrintString "SPEED SET")))

(event EventTick
  (params (DeltaSeconds :type Float%20%28single-precision%29))
  (bind _playerref (Variables|Default|GetPlayerRef))
  (bind _playerref_2 (Variables|Default|GetPlayerRef))
  (bind _charactermovement (Variables|/Script/Engine.Character|GetCharacterMovement _playerref))
  (bind _charactermovement_2 (Variables|/Script/Engine.Character|GetCharacterMovement _playerref_2))
  (switch int (Variables|Default|GetSetSpeed)
    (:0
      (Variables|/Script/Engine.CharacterMovementComponent|SetMaxWalkSpeed _charactermovement (Math|Interpolation|FInterptoConstant (Variables|/Script/Engine.CharacterMovementComponent|GetMaxWalkSpeed _charactermovement) (Variables|Default|GetMaxSpeedReset) DeltaSeconds 2e+01)))
    (:1
      (Variables|/Script/Engine.CharacterMovementComponent|SetMaxWalkSpeed _charactermovement_2 (Math|Interpolation|FInterptoConstant (Variables|/Script/Engine.CharacterMovementComponent|GetMaxWalkSpeed _charactermovement_2) (Variables|Default|GetMaxSpeedSet) DeltaSeconds 2e+01))
      (CallFunction|WIND))))

(event Collision|EventActorEndOverlap
  (params (OtherActor :type Actor%20Object%20Reference))
  (bind _sfx (Variables|Default|GetSFX))
  (if (and (== OtherActor (Game|Player|GetPlayerPawn 0)) (== (Variables|Default|GetSetSpeed) 1))
    (Variables|Default|SetSetSpeed 0)
    (Audio|Components|Audio|FadeOut _sfx 0.2 0.0 "Linear" :!class /Script/Engine.AudioComponent)
    (Utilities|FlowControl|Delay 5.0)
    (Components|DestroyComponent _sfx)))

(fn ConstructionScript)