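; Procedural world section that populates itself with enemies and triggers further generation as the player moves through it.
; On BeginPlay it spawns a few BP_Coronavirus actors at random points inside its SpawnEnemies box.
; The first time BP_FirstPersonCharacter overlaps its Box trigger, a DoOnce gate lets it call Generates on the BP_Manager found in the level.
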(event OnComponentBeginOverlap(Box)
  (params (OverlappedComponent :type Primitive%20Component%20Object%20Reference) (OtherActor :type Actor%20Object%20Reference) (OtherComp :type Primitive%20Component%20Object%20Reference) (OtherBodyIndex :type Integer) (bFromSweep :type Boolean) (SweepResult :type Hit%20Result%20Structure%20%28by%20ref%29))
  (Utilities|Casting|CastToBP_FirstPersonCharacter OtherActor)
  (Utilities|FlowControl|DoOnce false
    (:Completed
      (bind _returnvalue (Actor|GetActorOfClass "/Game/Blueprints/WorldGeneration/BP_Manager.BP_Manager_C"))
      (Default|Generates _returnvalue))))

(event EventBeginPlay
  (bind _spawnenemies (Variables|Default|GetSpawnEnemies))
  (|CallParentFunction)
  (for _index (range 0 3)
    (Variables|Default|SetSpawnEnemyRandomLocation (Math|Random|RandomPointinBoundingBox (Transformation|GetWorldLocation _spawnenemies) (Variables|/Script/Engine.BoxComponent|GetBoxExtent _spawnenemies)))
    (Game|SpawnActorfromClass "/Game/Blueprints/Enemy/BP_Coronavirus.BP_Coronavirus_C" (Math|Transform|MakeTransform (Variables|Default|GetSpawnEnemyRandomLocation) "0, 0, 0" "1.000000,1.000000,1.000000") "Undefined" "MultiplyWithRoot" 0 0)))

(event Collision|EventActorBeginOverlap
  (params (OtherActor :type Actor%20Object%20Reference))
  (|CallParentFunction OtherActor) ; This node is disabled and will not be called.\nDrag off pins to build functionality.
)

(event EventTick
  (params (DeltaSeconds :type Float%20%28single-precision%29))
  (|CallParentFunction DeltaSeconds) ; This node is disabled and will not be called.\nDrag off pins to build functionality.
)

(fn ConstructionScript
  (|CallParentFunction))