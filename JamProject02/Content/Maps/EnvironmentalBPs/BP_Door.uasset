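; BP_Door is an environmental door that lowers to open and rises to close along Z, using fixed world heights captured with its X/Y at BeginPlay.
; Switch alternates OpenDoor and CloseDoor through a FlipFlop, each setting a target and a move flag.
; Tick moves the mesh at constant speed until near that target.
; A hardcoded actor Y-position check makes only matching doors auto-close after a delay.
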(event Custom|Switch
  (Utilities|FlowControl|FlipFlop
    (:A
      (CallFunction|OpenDoor))
    (:B
      (CallFunction|CloseDoor))))

(event Custom|OpenDoor
  (Variables|Default|SetMoveTo (Variables|Default|GetOpen))
  (Variables|Default|SetbMove true)
  (if (== (.y (Transformation|GetActorLocation)) -5e+01)
    (Utilities|FlowControl|Delay 5.0)
    (CallFunction|CloseDoor)))

(event Custom|CloseDoor
  (Variables|Default|SetMoveTo (Variables|Default|GetClosed))
  (Variables|Default|SetbMove true))

(event EventTick
  (params (DeltaSeconds :type Float%20%28single-precision%29))
  (bind _staticmeshcomponent (Variables|Debug|GetStaticMeshComponent))
  (if (Variables|Default|GetbMove)
    (Transformation|SetWorldLocation _staticmeshcomponent (Math|Interpolation|VInterptoConstant (Transformation|GetWorldLocation _staticmeshcomponent) (Variables|Default|GetMoveTo) DeltaSeconds 1e+02) false false)
    (if (Utilities|Operators|EqualEqual (Transformation|GetWorldLocation _staticmeshcomponent) (Variables|Default|GetMoveTo) 2.0)
      (Variables|Default|SetbMove false))))

(event EventBeginPlay
  (bind _staticmeshcomponent (Variables|Debug|GetStaticMeshComponent))
  (bind _returnvalue (Transformation|GetWorldLocation _staticmeshcomponent))
  (Variables|Default|SetOpen (Math|Vector|MakeVector (.x _returnvalue) (.y _returnvalue) -4e+02))
  (Variables|Default|SetClosed (Math|Vector|MakeVector (.x _returnvalue) (.y _returnvalue) 0.0)))

(fn ConstructionScript)