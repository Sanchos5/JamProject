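; BP_FirstDoor is a one-shot door that starts open, sunk below the map, and closes after the player leaves its trigger.
; BeginPlay derives open and closed positions from the mesh's XY with fixed heights, then snaps it open.
; The first player end-overlap on R waits briefly, starts a constant-speed Tick interpolation to closed, then calls WAVESPAWNBEGIN on BP_ThirdPersonGameMode.
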(event OnComponentEndOverlap(r)
  (params (OverlappedComponent :type Primitive%20Component%20Object%20Reference) (OtherActor :type Actor%20Object%20Reference) (OtherComp :type Primitive%20Component%20Object%20Reference) (OtherBodyIndex :type Integer))
  (if (== OtherActor (Game|Player|GetPlayerPawn 0))
    (Utilities|FlowControl|DoOnce false
      (:Completed
        (Utilities|FlowControl|Delay 2.0)
        (CallFunction|CloseDoor)
        (Utilities|FlowControl|Delay 0.2)
        (bind _asbp_third_person_game_mode (Utilities|Casting|CastToBP_ThirdPersonGameMode (Game|GetGameMode)))
        (Default|WAVESPAWNBEGIN _asbp_third_person_game_mode)))))

(event Custom|OpenDoor
  (Transformation|SetWorldLocation (Variables|Debug|GetStaticMeshComponent) (Variables|Default|GetOpen) false false))

(event Custom|CloseDoor
  (Variables|Default|SetMoveTo (Variables|Default|GetClosed))
  (Variables|Default|SetbMove true))

(event EventTick
  (params (DeltaSeconds :type Float%20%28single-precision%29))
  (bind _staticmeshcomponent (Variables|Debug|GetStaticMeshComponent))
  (if (Variables|Default|GetbMove)
    (Transformation|SetWorldLocation _staticmeshcomponent (Math|Interpolation|VInterptoConstant (Transformation|GetWorldLocation _staticmeshcomponent) (Variables|Default|GetMoveTo) DeltaSeconds 1e+02) false false)
    (if (Utilities|Operators|EqualEqual (Transformation|GetWorldLocation _staticmeshcomponent) (Variables|Default|GetMoveTo) 2.0)
      (Variables|Default|SetbMove false))))

(event EventBeginPlay
  (bind _staticmeshcomponent (Variables|Debug|GetStaticMeshComponent))
  (bind _returnvalue (Transformation|GetWorldLocation _staticmeshcomponent))
  (Variables|Default|SetOpen (Math|Vector|MakeVector (.x _returnvalue) (.y _returnvalue) -4e+02))
  (Variables|Default|SetClosed (Math|Vector|MakeVector (.x _returnvalue) (.y _returnvalue) 0.0))
  (CallFunction|OpenDoor))

(fn ConstructionScript)