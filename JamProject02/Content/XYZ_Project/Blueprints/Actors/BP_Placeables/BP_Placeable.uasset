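; BP_Placeable is a placeable actor Blueprint with a timed lifespan.
; BeginPlay calls fLifespan, which uses a DoOnce to set a timer for fDestroyActor after Lifespan seconds and prints debug text.
; fDestroyActor prints and then calls itself through a DoOnce, with no actual DestroyActor call shown.
; An unconnected test node that moves and scales the Box component never runs.
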(event EventBeginPlay
  (CallFunction|FLifespan))

(fn ConstructionScript)

(fn FLifespan
  (bind _lifespan (Variables|Default|GetLifespan))
  (Utilities|FlowControl|DoOnce false
    (:Completed
      (Utilities|Time|SetTimerbyFunctionName 0 "fDestroyActor" _lifespan)
      (Development|PrintString (Utilities|String|BuildString(Float) "" "Timer Set: " _lifespan))
      (return))))

(fn FDestroyActor
  (Development|PrintString "DestroyActor")
  (Utilities|FlowControl|DoOnce false
    (:Completed
      (CallFunction|FDestroyActor))))