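; Placeable flower trap that periodically damages enemies in front of it, extending a parent class with lifespan and destroy logic.
; Its damage zone locks onto one enemy through a DoOnce, releasing it when that enemy leaves.
; Tick smoothly yaws the flower toward the target, or spins it passively in the last stored direction.
; A looping timer capsule-traces from the muzzle, applying point damage to enemy-base children and fading in the damage sound.
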(event OnComponentBeginOverlap(DamageZone)
  (params (OverlappedComponent :type Primitive%20Component%20Object%20Reference) (OtherActor :type Actor%20Object%20Reference) (OtherComp :type Primitive%20Component%20Object%20Reference) (OtherBodyIndex :type Integer) (bFromSweep :type Boolean) (SweepResult :type Hit%20Result%20Structure%20%28by%20ref%29))
  ;[1 1 1] set target
  ;;[1 1 1] target is child of enemy base
  (if (Utilities|ClassIsChildOf (Utilities|GetClass OtherActor) "/Game/XYZ_Project/AI/Enemies/AIclassBASEs/BP_Enemy_BASE.BP_Enemy_BASE_C")
    (Utilities|FlowControl|DoOnce false
      (:Completed
        (bind _output_get (Variables|Default|SetTarget OtherActor))
        (Variables|Default|SetTargetSet true)
        ;;[1 1 1] debug
        (Development|PrintString (Utilities|String|BuildString(Object) "" "Flower Target: " _output_get " Target Set"))))))

(event OnComponentEndOverlap(DamageZone)
  (params (OverlappedComponent :type Primitive%20Component%20Object%20Reference) (OtherActor :type Actor%20Object%20Reference) (OtherComp :type Primitive%20Component%20Object%20Reference) (OtherBodyIndex :type Integer))
  ;[1 1 1] set target
  ;;[1 1 1] follows a single target
  (if (== OtherActor (Variables|Default|GetTarget))
    (Variables|Default|SetTargetSet false)
    (Utilities|FlowControl|DoOnce false) ; enters at Reset
  ))

(event EventBeginPlay
  ;[1 1 1] f lifespan
  (|CallParentFunction)
  (Utilities|Time|SetTimerbyFunctionName 0 "fDamageToActorInFront" (Variables|Default|GetTimeBetweenAttacks) true)
  (Audio|Components|Audio|SetVolumeMultiplier (Variables|Default|GetDamageSound) 0.0 :!class /Script/Engine.AudioComponent))

(event EventTick
  (params (DeltaSeconds :type Float%20%28single-precision%29))
  (bind _self self)
  (bind _self_2 self)
  (bind _target (Variables|Default|GetTarget))
  (bind _returnvalue (Transformation|GetActorLocation _target))
  (bind _defaultsceneroot (Variables|Default|GetDefaultSceneRoot _self_2))
  (bind _defaultsceneroot_2 (Variables|Default|GetDefaultSceneRoot _self))
  (bind _returnvalue_2 (Transformation|GetWorldRotation _defaultsceneroot))
  (bind _returnvalue_3 (Transformation|GetWorldLocation _defaultsceneroot_2))
  (bind _returnvalue_4 (Transformation|GetWorldRotation _defaultsceneroot_2))
  (bind _returnvalue_5 (Math|Rotator|FindLookatRotation _returnvalue_3 _returnvalue))
  (bind _returnvalue_6 (Math|Interpolation|RInterpTo (Math|Rotator|MakeRotator 0.0 0.0 (.yaw _returnvalue_4)) (Math|Rotator|MakeRotator 0.0 0.0 (.yaw _returnvalue_5)) DeltaSeconds 0.0))
  ;[1 1 1] event tick
  (if (not (Variables|Default|GetTargetSet))
    ;[1 1 1] passive rotation
    (Transformation|SetWorldRotation _defaultsceneroot (Math|Interpolation|RInterpTo (Math|Rotator|MakeRotator 0.0 0.0 (.yaw _returnvalue_2)) (Math|Rotator|MakeRotator 0.0 0.0 (+ (.yaw _returnvalue_2) (* (Variables|Default|GetAddRotation) (Variables|Default|GetRotationDirection)))) DeltaSeconds 0.0) false false)
    (else
      ;[1 1 1] rotate to target
      ;;[1 1 1] set rotation direction (+ = clockwise)
      (if (>= (.yaw _returnvalue_6) 0.0)
        (Variables|Default|SetRotationDirection 1.0)
        (else
          (Variables|Default|SetRotationDirection -1.0)))
      (Transformation|SetWorldRotation (Variables|Default|GetDefaultSceneRoot self) (Math|Rotator|MakeRotator 0.0 0.0 (.yaw _returnvalue_6)) false false))))

(fn ConstructionScript
  (|CallParentFunction))

(fn FLifespan
  (|CallParentFunction))

(fn FDestroyActor
  (|CallParentFunction))

(fn FDamagetoActorinFront
  (bind _muzzle (Variables|Default|Getmuzzle))
  (bind _damagesound (Variables|Default|GetDamageSound))
  (bind _returnvalue (Transformation|GetSocketTransform _muzzle "None" "RTS_World"))
  ;[1 1 1] check if there is an actor in front of the trap
  (bind _outhit (Collision|CapsuleTraceByChannel (.location _returnvalue) (+ (.location _returnvalue) (* (Math|Vector|GetForwardVector (.rotation _returnvalue)) 3e+02)) 1.5e+02 1.5e+02 "TraceTypeQuery1" false 0 "None"))
  ;[1 1 1] apply damage only to children of enemy base
  (if (Utilities|ClassIsChildOf (Utilities|GetClass (.HitActor (Collision|BreakHitResult _outhit))) "/Game/XYZ_Project/AI/Enemies/AIclassBASEs/BP_Enemy_BASE.BP_Enemy_BASE_C")
    (bind _returnvalue_2 (Game|Damage|ApplyPointDamage (.HitActor (Collision|BreakHitResult _outhit)) (Variables|Default|GetDamagePerAttack) (.ImpactPoint (Collision|BreakHitResult _outhit)) _outhit))
    (Audio|Components|Audio|SetVolumeMultiplier _damagesound 1.0 :!class /Script/Engine.AudioComponent)
    (Audio|Components|Audio|FadeIn _damagesound 0.1 0.2 0.0 "Linear" :!class /Script/Engine.AudioComponent)))