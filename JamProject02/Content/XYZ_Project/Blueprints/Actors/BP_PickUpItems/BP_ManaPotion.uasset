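; Mana potion pickup that refills reserve ammo for the player's fire staff and electro knife when its AddAmmo event fires.
; The pickup function casts each weapon child actor separately, adds magazine size times a reload multiplier clamped to max ammo, and calls its fire animation.
; Each successful branch sets a timer for fDestroyActor, which is empty here; the parent pickup logic is never called.
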(event Custom|AddAmmo
  (params (PlayerCharacter :type BP%20Player%20Character%20Object%20Reference))
  (CallFunction|FPickUpItem PlayerCharacter "0, 0, 0" "0, 0, 0" 0 false))

(fn ConstructionScript
  (|CallParentFunction))

(fn FPickUpItem
  (params (PlayerCharacter :type BP%20Player%20Character%20Object%20Reference) (EmitterLoc :type Vector :default "0, 0, 0") (EmitterRotation :type Rotator :default "0, 0, 0") (AttachToComponent :type Scene%20Component%20Object%20Reference) (StopEffects :type Boolean))
  (Utilities|FlowControl|Sequence
    (:then_0
      (bind _asbp_ebfire_staff (Utilities|Casting|CastToBP_EBFireStaff (Variables|/Script/Engine.ChildActorComponent|GetChildActor (Variables|/Game/XYZ_Project/Core/Character/Player/BP_PlayerCharacter.BP_PlayerCharacter_C|Getstaff%20actor PlayerCharacter))))
      (bind _ammoinposession (Default|GetAmmo _asbp_ebfire_staff))
      ;[1 1 1] potion grants reloadmultiplier*weaponammomag amount of ammo
      (bind _output_get (Variables|Default|SetAmmoToReload (Math|Float|Truncate (* (Variables|/Game/XYZ_Project/Weapons/BP_EBFireStaff.BP_EBFireStaff_C|GetMagSize%20FireStaff _asbp_ebfire_staff) (Variables|Default|GetReloadMultiplier)))))
      (Variables|/Game/XYZ_Project/Weapons/BP_EBPlayerWeapon_BASE.BP_EBPlayerWeapon_BASE_C|SetAmmoInPosession _asbp_ebfire_staff (Math|Integer|Clamp(Integer) (+ _ammoinposession _output_get) 0 (Variables|/Game/XYZ_Project/Weapons/BP_EBFireStaff.BP_EBFireStaff_C|GetMaxAmmo%20FireStaff _asbp_ebfire_staff)))
      (Default|PlayFireAnimation _asbp_ebfire_staff))
    (:then_1
      (bind _asbp_ebknife (Utilities|Casting|CastToBP_EBKnife (Variables|/Script/Engine.ChildActorComponent|GetChildActor (Variables|/Game/XYZ_Project/Core/Character/Player/BP_PlayerCharacter.BP_PlayerCharacter_C|Getknife%20actor PlayerCharacter))))
      (bind _ammoinposession_2 (Default|GetAmmo _asbp_ebknife))
      (bind _output_get_2 (Variables|Default|SetAmmoToReload (Math|Float|Truncate (* (Variables|/Game/XYZ_Project/Weapons/BP_EBKnife.BP_EBKnife_C|GetMagsizeElectroKnife _asbp_ebknife) (Variables|Default|GetReloadMultiplier)))))
      (Variables|/Game/XYZ_Project/Weapons/BP_EBPlayerWeapon_BASE.BP_EBPlayerWeapon_BASE_C|SetAmmoInPosession _asbp_ebknife (Math|Integer|Clamp(Integer) (+ _ammoinposession_2 _output_get_2) 0 (Variables|/Game/XYZ_Project/Weapons/BP_EBKnife.BP_EBKnife_C|GetMaxAmmoElectroKnife _asbp_ebknife)))
      (Default|PlayFireAnimation _asbp_ebknife)))
  (Utilities|Time|SetTimerbyFunctionName 0 "fDestroyActor" (Variables|Default|GetTimer)))

(fn FDestroyActor)