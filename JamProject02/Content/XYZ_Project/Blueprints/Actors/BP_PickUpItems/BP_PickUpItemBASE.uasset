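; Base actor for pickup items that handles pickup sound and particle effects and a temporary "item maxed" indicator.
; The item's sound is muted at BeginPlay; the pickup function restores volume, fades it in and spawns an attached emitter unless the effects timer is active.
; An optional timer calls EffectsStop to fade the sound out and destroy the particle component.
; CannotPickItemUp briefly shows the ItemMaxed component.
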(event Custom|EffectsStop
  (bind _particlesystemref (Variables|Default|GetParticleSystemRef))
  (Audio|Components|Audio|FadeOut (Variables|Default|GetItemCue) 0.1 0.2 "Linear" :!class /Script/Engine.AudioComponent)
  (Components|Activation|Deactivate _particlesystemref)
  (Components|DestroyComponent _particlesystemref))

(event Custom|CannotPickItemUp
  (bind _itemmaxed (Variables|Default|GetItemMaxed))
  (Rendering|SetVisibility _itemmaxed true false)
  (Utilities|FlowControl|Delay 1.5)
  (Rendering|SetVisibility _itemmaxed false false))

(event EventBeginPlay
  (bind _itemcue (Variables|Default|GetItemCue))
  (Utilities|IsValid _itemcue
    (:Is%20Valid
      (Audio|Components|Audio|SetVolumeMultiplier _itemcue 0.0 :!class /Script/Engine.AudioComponent))))

(fn ConstructionScript)

(fn FPickUpItem
  (params (PlayerCharacter :type BP%20Player%20Character%20Object%20Reference) (EmitterLoc :type Vector) (EmitterRotation :type Rotator) (AttachToComponent :type Scene%20Component%20Object%20Reference) (StopEffects :type Boolean))
  ;[1 1 1] spawn effects
  (if (Utilities|Time|IsTimerActivebyHandle (Variables|Default|GetEffectsTimer))
    (return)
    (else
      (CallFunction|FItemEffects (Variables|Default|GetItemCue) (Variables|Default|GetEmitter) EmitterLoc (Variables|Default|GetEmitterScale) EmitterRotation AttachToComponent)
      ;[1 1 1] stop effects
      (if StopEffects
        (bind _returnvalue (Utilities|Time|SetTimerbyFunctionName 0 "EffectsStop" (Variables|Default|GetTimer)))
        (Variables|Default|SetEffectsTimer _returnvalue)
        (else
          (return))))))

(fn FItemEffects
  (params (SoundCue :type Audio%20Component%20Object%20Reference) (Emitter :type Particle%20System%20Object%20Reference) (EmitterLoc :type Vector) (EmitterScale :type Vector) (EmitterRotation :type Rotator) (AttachToComponent :type Scene%20Component%20Object%20Reference))
  (Audio|Components|Audio|SetVolumeMultiplier SoundCue 1.0 :!class /Script/Engine.AudioComponent)
  (Audio|Components|Audio|FadeIn SoundCue 0.1 0.2 0.0 "Linear" :!class /Script/Engine.AudioComponent)
  (bind _returnvalue (Effects|SpawnEmitterAttached Emitter AttachToComponent "" EmitterLoc EmitterRotation EmitterScale))
  (Variables|Default|SetParticleSystemRef _returnvalue))

(fn FEffectsStop)