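; Base character Blueprint that handles health, damage and death, with health set to maximum on BeginPlay.
; AnyDamage passes damage through FGetHP, which clamps health and flags death at zero, then into FDeath.
; FDeath plays the death montage on the mesh and calls CallActorDeath behind a DoOnce, though a comment notes it fires twice for enemies.
; FGetHealthRatio exposes normalized health; OnDeath is an empty event.
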(event Custom|OnDeath)

(event Game|Damage|EventAnyDamage
  (params (Damage :type Float%20%28single-precision%29) (DamageType :type Damage%20Type%20Object%20Reference) (InstigatedBy :type Controller%20Object%20Reference) (DamageCauser :type Actor%20Object%20Reference))
  (if (not (Variables|HP|GetbIsDead))
    (bind _bisdead (CallFunction|FGetHP (Variables|HP|GetCurrentHealth) Damage))
    (CallFunction|FDeath _bisdead (Variables|Character|GetMesh) (Variables|HP|GetDeathMontage))))

(event EventBeginPlay
  (Variables|HP|SetCurrentHealth (Variables|HP|GetMaxHealth)))

(fn ConstructionScript)

(fn FGetHealthRatio
  (bind _output_get (Variables|HP|SetHealthRatio (Math|Float|Clamp(Float) (/ (Variables|HP|GetCurrentHealth) (Variables|HP|GetMaxHealth)))))
  (return _output_get))

(fn FGetHP
  (params (ActorHealth :type Float%20%28single-precision%29) (DamageReceived :type Float%20%28single-precision%29))
  (Variables|HP|SetCurrentHealth ActorHealth)
  (if (> (Variables|HP|GetCurrentHealth) 0.0)
    (bind _output_get (Variables|HP|SetCurrentHealth (Math|Float|Clamp(Float) (- (Variables|HP|GetCurrentHealth) DamageReceived) 0.0 (Variables|HP|GetMaxHealth))))
    (if (== _output_get 0.0)
      _
      (else
        (return (Variables|HP|GetCurrentHealth) false))))
  (Utilities|FlowControl|DoOnce false
    (:Completed
      (bind _output_get_2 (Variables|HP|SetbIsDead true))
      (return 0.0 _output_get_2))))

(fn FDeath
  (params (bIsDead :type Boolean) (ActorMesh :type Skeletal%20Mesh%20Component%20Object%20Reference) (DeathMontage :type Anim%20Montage%20Object%20Reference))
  (if bIsDead
    (Utilities|IsValid ActorMesh
      (:Is%20Valid
        (Utilities|FlowControl|DoOnce false
          (:Completed
            (Animation|Montage|MontagePlay (Components|SkeletalMesh|GetAnimInstance ActorMesh) DeathMontage 1.0 "MontageLength" 0.0 true)
            ;[1 1 1] is called twice per bp enemy actor death for some reason
            (Default|CallActorDeath)
            (return)))))))