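; Base weapon Blueprint built around an EBarrel component, sketching magazine and reserve-ammo reloading.
; The reload logic blocks shooting, computes missing rounds, refills the barrel from reserve ammo, then unblocks it.
; All of that logic, including debug printouts, is disconnected and never runs.
; Tick, GetRequiredAmmo and IsReloadRequired are empty, and the construction script only calls its parent.
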(event Custom|GetRequiredAmmo
  ;[1 1 1] Ammo Counting and Reload
  ;;[1 1 1] RequiredAmmo
)

(event Custom|IsReloadRequired
  ;[1 1 1] Ammo Counting and Reload
  ;;[1 1 1] IsReloadRequired
)

(event EventTick
  (params (DeltaSeconds :type Float%20%28single-precision%29))
  ;[1 1 1] Ammo Counting and Reload
)

(fn ConstructionScript
  (|CallParentFunction))