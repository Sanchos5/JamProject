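; Base enemy projectile that keeps the level's enemies in its ignored-actor list so enemies don't damage each other.
; On BeginPlay it casts the game mode to BP_BasicGameMode and copies AllEnemiesOnLevel into IgnoredActors.
; It also binds to the game mode's enemy list update event, refreshing the ignored list whenever that event fires.
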(event Custom|UpdateIgnoredActors
  ;[1 1 1] enemies don't damage each other
  (Variables|Default|SetIgnoredActors (Variables|/Game/XYZ_Project/Core/Framework/BP_BasicGameMode.BP_BasicGameMode_C|GetAllEnemiesOnLevel (Variables|Default|GetGameModeRef))))

(event EventBeginPlay
  ;[1 1 1] enemies don't damage each other
  (bind _asbp_basic_game_mode (Utilities|Casting|CastToBP_BasicGameMode (Game|GetGameMode)))
  (bind _output_get (Variables|Default|SetGameModeRef _asbp_basic_game_mode))
  (Variables|Default|SetIgnoredActors (Variables|/Game/XYZ_Project/Core/Framework/BP_BasicGameMode.BP_BasicGameMode_C|GetAllEnemiesOnLevel _output_get))
  (EventDispatchers|BindEventtoEnemiesonLevelUpdate _output_get (delegate Custom|UpdateIgnoredActors)))

(fn ConstructionScript
  (|CallParentFunction))