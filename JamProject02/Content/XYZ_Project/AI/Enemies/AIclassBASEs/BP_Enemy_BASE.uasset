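; Base enemy Blueprint that extends inherited health and death logic with hit reactions, a health bar and coin drops.
; Non-lethal damage targets the player through the AI controller reference and temporarily shows the health bar, which Tick yaws toward the player.
; Death plays through the parent function, hides the bar, may spawn a valued coin after a delay, then destroys the body.
; Comments note that child classes must set up the health bar individually.
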(event EventBeginPlay
  ;[1 1 1] event BeginPlay
  (Utilities|FlowControl|Sequence
    (:then_0
      ;[1 1 1] wbp healthbar doesn't work for children classes of enemy base. set individually in each ai enemy class
      (bind _aswbp_healthbar (Utilities|Casting|CastToWBP_Healthbar (UserInterface|GetUserWidgetObject (Variables|Default|GetHealthbar)))
        (:then
          (bind _output_get (Variables|/Game/XYZ_Project/Widgets/UserInterface/Bars/WBP_Healthbar.WBP_Healthbar_C|SetWidgetOwnerRef _aswbp_healthbar self))
          (Variables|References|SetHealthBarRef _aswbp_healthbar)
          (Rendering|SetVisibility (Variables|Default|GetHealthbar) false false))
        (:CastFailed
          ;;[1 1 1] debug
          (Development|PrintString "Cast to Widget Healthbar Invalid"))))))

(event EventTick
  (params (DeltaSeconds :type Float%20%28single-precision%29))
  (bind _healthbar (Variables|Default|GetHealthbar))
  ;[1 1 1] Healthbar Visibility and TurnToPlayer
  (if (Rendering|IsVisible (Variables|Default|GetHealthbar))
    ;;[1 1 1] bar rotates to player
    (Transformation|SetWorldRotation _healthbar (Math|Rotator|MakeRotator 0.0 0.0 (.yaw (Math|Rotator|FindLookatRotation (Transformation|GetWorldLocation _healthbar) (Transformation|GetActorLocation (Game|GetPlayerCharacter 0))))) false false)
    (else
      (Utilities|FlowControl|Delay 2.0)
      (Rendering|SetVisibility (Variables|Default|GetHealthbar) false false))))

(event Game|Damage|EventAnyDamage
  (params (Damage :type Float%20%28single-precision%29) (DamageType :type Damage%20Type%20Object%20Reference) (InstigatedBy :type Controller%20Object%20Reference) (DamageCauser :type Actor%20Object%20Reference))
  ;[1 1 1] Health
  (Animation|Montage|MontagePlay (Components|SkeletalMesh|GetAnimInstance (Variables|Character|GetMesh)) (Variables|AnimMontages|GetHitMontage) 1.3 "MontageLength" 0.0 true)
  (|CallParentFunction Damage 0 0 0)
  (if (Variables|Default|GetbIsDead)
    ;;[1 1 1] death additions
    (CallFunction|FDeath true (Variables|Character|GetMesh) (Variables|Default|GetDeathMontage))
    ;;;[1 1 1] wbp
    (Rendering|SetVisibility (Variables|Default|GetHealthbar) false false)
    (Utilities|FlowControl|Delay 4.0)
    ;;;[1 1 1] with a random chance spawn coin after actor death
    (bind _output_get (Variables|Coins|SetRandomChance (Math|Random|RandomFloatinRange 0.0 1e+02)))
    (if (<= _output_get (Variables|Coins|GetCoinSpawnChance))
      (bind _returnvalue (Game|SpawnActorfromClass "/Game/XYZ_Project/Blueprints/Actors/BP_PickUpItems/BP_Coin.BP_Coin_C" (Transformation|GetWorldTransform (Variables|Transformation|GetRootComponent self)) "AdjustIfPossibleButAlwaysSpawn" 0 0))
      (Variables|/Game/XYZ_Project/Blueprints/Actors/BP_PickUpItems/BP_Coin.BP_Coin_C|SetCoinValue _returnvalue (Variables|Coins|GetEnemyCoinValue)))
    ;;;[1 1 1] let the body lie on the floor a little
    (Utilities|FlowControl|Delay 5.0)
    (Actor|DestroyActor)
    (else
      ;;[1 1 1] AI alive after getting hit, set player as target
      (Default|SetTargetEnemy (Variables|References|GetAICBaseRef) (Game|GetPlayerCharacter 0))
      ;;[1 1 1] wbp healthbar
      (Rendering|SetVisibility (Variables|Default|GetHealthbar) true false)
      (Utilities|FlowControl|Delay 1e+01)
      (Rendering|SetVisibility (Variables|Default|GetHealthbar) false false))))

(fn ConstructionScript)

(fn FGetHP
  (params (ActorHealth :type Float%20%28single-precision%29) (DamageReceived :type Float%20%28single-precision%29))
  (bind (_currenthealth _bisdead) (|CallParentFunction ActorHealth DamageReceived))
  (return _currenthealth _bisdead))

(fn FDeath
  (params (bIsDead :type Boolean) (ActorMesh :type Skeletal%20Mesh%20Component%20Object%20Reference) (DeathMontage :type Anim%20Montage%20Object%20Reference))
  (|CallParentFunction bIsDead ActorMesh DeathMontage))

(fn FGetHealthRatio
  (bind _healthratio (|CallParentFunction))
  (return _healthratio))