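; BP_MeleeWeaponBASE is a melee weapon base for enemy AI that damages what its hitbox touches.
; On overlap, a living BP_Enemy_BASE owner applies point damage of type DT_AIWeapon to non-enemy actors and plays AttackCue.
; A DoOnce gate limits this to one hit until an overlap ends; the end-overlap check compares OtherActor to itself, so any actor leaving resets it.
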(event OnComponentBeginOverlap(WeaponHitbox)
  (params (OverlappedComponent :type Primitive%20Component%20Object%20Reference) (OtherActor :type Actor%20Object%20Reference) (OtherComp :type Primitive%20Component%20Object%20Reference) (OtherBodyIndex :type Integer) (bFromSweep :type Boolean) (SweepResult :type Hit%20Result%20Structure%20%28by%20ref%29))
  (bind _weaponowner (Variables|Default|GetWeaponOwner))
  (bind _attackcue (Variables|Default|GetAttackCue))
  ;[1 1 1] apply damage on hitbox overlap
  ;;[1 1 1] enemy ai applies damage when alive and doesn't damage other enemies
  (if (and (Utilities|ClassIsChildOf (Utilities|GetClass _weaponowner) "/Game/XYZ_Project/AI/Enemies/AIclassBASEs/BP_Enemy_BASE.BP_Enemy_BASE_C") (not (Variables|/Game/XYZ_Project/Core/Character/BP_BaseCharacter.BP_BaseCharacter_C|GetbIsDead _weaponowner)))
    (if (not (Utilities|ClassIsChildOf (Utilities|GetClass OtherActor) "/Game/XYZ_Project/AI/Enemies/AIclassBASEs/BP_Enemy_BASE.BP_Enemy_BASE_C"))
      ;;[1 1 1] applies damage only once on hitbox breach, reset upon hitbox everlap ending
      (Utilities|FlowControl|DoOnce false
        (:Completed
          (Game|Damage|ApplyPointDamage OtherActor (Variables|Default|GetHitDamage) (Transformation|GetWorldLocation (Variables|Default|GetWeaponHitbox)) SweepResult 0 self "/Game/XYZ_Project/Weapons/DamageTypes/DT_AIWeapon.DT_AIWeapon_C")
          (Audio|Components|Audio|SetVolumeMultiplier _attackcue 0.1 :!class /Script/Engine.AudioComponent)
          (Audio|Components|Audio|Play _attackcue 0.0))))))

(event OnComponentEndOverlap(WeaponHitbox)
  (params (OverlappedComponent :type Primitive%20Component%20Object%20Reference) (OtherActor :type Actor%20Object%20Reference) (OtherComp :type Primitive%20Component%20Object%20Reference) (OtherBodyIndex :type Integer))
  (bind _attackcue (Variables|Default|GetAttackCue))
  ;[1 1 1] apply damage on hitbox overlap
  ;;[1 1 1] reset apply damage on end component overlap
  (if (== (stale OnComponentBeginOverlap(WeaponHitbox) OtherActor) OtherActor)
    ;;[1 1 1] applies damage only once on hitbox breach, reset upon hitbox everlap ending
    (Utilities|FlowControl|DoOnce false) ; enters at Reset
  ))

(event EventBeginPlay
  (Audio|Components|Audio|SetVolumeMultiplier (Variables|Default|GetAttackCue) 0.0 :!class /Script/Engine.AudioComponent))

(fn ConstructionScript)