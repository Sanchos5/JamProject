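; Base projectile Blueprint that applies damage on impact for both AI and player weapons, branching on the projectile's owner.
; An owner that casts to BP_EBWeaponBASE deals point damage from that weapon's stats with the AI weapon damage type.
; Any other valid owner, intended as the player weapon, uses the projectile's own stats for point and radial damage, plus an emitter scaled to splash radius.
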(event EventOnImpact
  (params (Ricochet :type Boolean) (PassedThrough :type Boolean) (Location :type Vector :default "0, 0, 0") (IncomingVelocity :type Vector :default "0, 0, 0") (Normal :type Vector :default "0, 0, 0") (ExitLocation :type Vector :default "0, 0, 0") (ExitVelocity :type Vector :default "0, 0, 0") (Impulse :type Vector :default "0, 0, 0") (PenetrationDepth :type Float%20%28double-precision%29) (Actor :type Actor%20Object%20Reference) (Component :type Scene%20Component%20Object%20Reference) (BoneName :type Name :default "None") (PhysMaterial :type Physical%20Material%20Object%20Reference) (HitResult :type Hit%20Result%20Structure))
  (bind _returnvalue (Math|Vector|Normalize IncomingVelocity))
  (bind _returnvalue_2 (Components|GetOwner))
  (bind _splashradius (Variables|Damage|GetSplashRadius))
  (bind _returnvalue_3 (/ _splashradius 2.5e+02))
  ;[1 1 1] ProjectileImpact
  ;;[1 1 1] weaponbase path aka AI Weapons and Projectiles
  (Utilities|IsValid _returnvalue_2
    (:Is%20Valid
      (bind _asbp_ebweapon_base (Utilities|Casting|CastToBP_EBWeaponBASE _returnvalue_2)
        (:then
          (bind _output_get (Variables|EBullet|SetWeaponBASERef _asbp_ebweapon_base))
          (Game|Damage|ApplyPointDamage Actor (* (Variables|/Game/MIGRATED/Weapons/GeneralClassBASES/BP_EBWeaponBASE.BP_EBWeaponBASE_C|GetDamage _output_get) (Variables|/Game/MIGRATED/Weapons/GeneralClassBASES/BP_EBWeaponBASE.BP_EBWeaponBASE_C|GetPointMultiplier _output_get)) _returnvalue HitResult 0 0 "/Game/MIGRATED/Weapons/DamageTypes/DT_AIWeapon.DT_AIWeapon_C"))
        (:CastFailed
          ;;[1 1 1] roundabout since playerweapon class is not based off of ebweaponbase
          (Effects|SpawnEmitteratLocation 0 Location "0, 0, 0" (Math|Vector|MakeVector _returnvalue_3 _returnvalue_3 _returnvalue_3))
          (Game|Damage|ApplyPointDamage Actor (Math|Conversions|ToFloat(Integer) (Math|Float|Round (* (Variables|Damage|GetDamage) (Variables|Damage|GetPointMultiplier)))) _returnvalue HitResult)
          (Game|Damage|ApplyRadialDamage (Math|Conversions|ToFloat(Integer) (Math|Float|Round (* (Variables|Damage|GetDamage) (Variables|Damage|GetSplashMultiplier)))) Location (Variables|Damage|GetSplashRadius) 0 0 0 0 false "ECC_Visibility"))))))

(fn ConstructionScript)