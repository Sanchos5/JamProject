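; Base game mode that spawns timed waves of random enemies at BP_SpawnPoint locations.
; BeginPlay caches spawn points and starts SpawnWave, which restarts the wave timer until the wave limit.
; SetAllEnemiesOnLevel appends non-mannequin BP_Enemy_BASE actors to an array, setting looping timers to the empty KillCounterWin event.
; Kill-count win logic and player-death binding to CloseGame, which opens MainMenu, are disconnected.
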(event Custom|KillCounterWin
  ;[1 1 1] Kill Mission Objective
  ;;[1 1 1] kill all enemies on level
)

(event Custom|CloseGame
  ;[1 1 1] PlayerDead Gameover Rule
  (Utilities|FlowControl|Delay 3.0)
  (Game|OpenLevel(byName) "MainMenu"))

(event Custom|EnemyWaveTimer
  ;[1 1 1] SpawnWave
  (bind _returnvalue (Utilities|Time|SetTimerbyEvent (delegate Custom|SpawnWave) (Variables|WaveSpawnVariables|GetTimeBetweenWaves) true))
  (Variables|WaveSpawnVariables|SetWaveTimer _returnvalue))

(event Custom|SpawnWave
  (bind _spawnpoints (Variables|WaveSpawnVariables|GetSpawnPoints))
  (bind _enemytypes (Variables|EnemyVariables|GetEnemyTypes))
  ;[1 1 1] SpawnWave
  ;;[1 1 1] check if there are waves left  to spawn
  (if (< (Variables|WaveSpawnVariables|GetWaveCounter) (Variables|WaveSpawnVariables|GetNumberOfWavesToSpawn))
    ;;[1 1 1] debug
    (Development|PrintString "SPAWNWAVE" true true "(R=0.000000,G=1.000000,B=0.051529,A=1.000000)" 4.0)
    ;;[1 1 1] set wave counter and reset timer
    (Utilities|Time|ClearandInvalidateTimerbyHandle (Variables|WaveSpawnVariables|GetWaveTimer))
    (Variables|WaveSpawnVariables|SetWaveCounter (+ (Variables|WaveSpawnVariables|GetWaveCounter) 1.0))
    ;;[1 1 1] get info about enemies to spawn
    (bind _output_get (Variables|WaveSpawnVariables|SetN%20Enemies (Math|Random|RandomIntegerinRange 0 (- (Variables|WaveSpawnVariables|GetMaxNumberOfEnemiesInWave) 1))))
    (for _index (range 0 _output_get)
      ;;[1 1 1] spawn location
      (bind _returnvalue (Game|SpawnActorfromClass (Utilities|Array|Get(acopy) _enemytypes (Math|Random|RandomIntegerinRange 0 (- (Utilities|Array|Length _enemytypes) 1))) (Utilities|Array|Get(acopy) _spawnpoints (Math|Random|RandomIntegerinRange 0 (- (Utilities|Array|Length _spawnpoints) 1))) "Undefined" "SelectDefaultAtRuntime" 0 0)))
    ;;[1 1 1] reset enemy wave timer after spawning actors and add them to the allenemies array
    (CallFunction|EnemyWaveTimer)
    (bind _allenemiesonlevel (CallFunction|SetAllEnemiesonLevel (delegate Custom|KillCounterWin)))
    (else
      (Development|PrintString "No More Waves To Spawn" true true "(R=0.964954,G=1.000000,B=0.000000,A=1.000000)" 4.0))))

(event EventBeginPlay
  (Utilities|FlowControl|Sequence
    (:then_0
      ;[1 1 1] Kill Mission Objective
      ;;[1 1 1] kill all enemies on level
      (Utilities|FlowControl|Sequence
        (:then_0
          (CallFunction|SetAllEnemiesonLevel (delegate Custom|KillCounterWin)))
        (:then_1
          ;;[1 1 1] set up enemy spawn locations array
          (bind _outactors (Actor|GetAllActorsOfClass "/Game/MIGRATED/Blueprints/WaveSpawner/BP_SpawnPoint.BP_SpawnPoint_C"))
          (for _array_element _outactors
            (Utilities|Array|Add (Variables|WaveSpawnVariables|GetSpawnPoints) (Variables|/Game/MIGRATED/Blueprints/WaveSpawner/BP_SpawnPoint.BP_SpawnPoint_C|GetSpawnLocation _array_element))))))
    (:then_1
      ;[1 1 1] SpawnWave
      ;;[1 1 1] if BuildingObjective is present on level then set WaveTimer
      (CallFunction|EnemyWaveTimer)
      (CallFunction|SpawnWave))))

(fn ConstructionScript)

(fn SetAllEnemiesonLevel
  (params (Event%20To%20Bind%20To%20Actor%20Death :type Delegate%20%28by%20ref%29))
  (bind _outactors (Actor|GetAllActorsOfClass "/Game/MIGRATED/AI/Enemies/AIclassBASEs/BP_Enemy_BASE.BP_Enemy_BASE_C"))
  (for _array_element _outactors
    ;[1 1 1] exclude mannequins
    (if (!= (Utilities|GetClass _array_element) "/Game/MIGRATED/AI/Enemies/AI_Mannequin.AI_Mannequin_C")
      (Utilities|Array|Add (Variables|EnemyVariables|GetAllEnemiesOnLevel) _array_element)
      (Utilities|Time|SetTimerbyEvent Event%20To%20Bind%20To%20Actor%20Death 2.0 true)))
  ;[1 1 1] enemy on level counter
  (Development|PrintString (Utilities|String|BuildString(Integer) "" "Enemies On Level " (Utilities|Array|Length (Variables|EnemyVariables|GetAllEnemiesOnLevel))) true true "(R=1.000000,G=0.762087,B=0.000000,A=1.000000)" 5.0)
  (return (Variables|EnemyVariables|GetAllEnemiesOnLevel)))