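; Health potion pickup, a child of a shared pick-up item Blueprint, that restores the player character's health.
; The Heal event runs the pick-up function, which adds HealHP to current health, clamped between zero and max health.
; It then calls the parent pick-up, passing the player's capsule as the attach component and a flag to stop effects.
; The destroy-actor override is empty.
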(event Custom|Heal
  (params (PlayerCharacter :type %20Object%20Reference))
  (CallFunction|FPickUpItem PlayerCharacter "0, 0, 0" "0, 0, 0" 0 true))

(fn ConstructionScript
  (|CallParentFunction))

(fn FPickUpItem
  (params (PlayerCharacter :type %20Object%20Reference) (EmitterLoc :type Vector :default "0, 0, 0") (EmitterRotation :type Rotator :default "0, 0, 0") (AttachToComponent :type Scene%20Component%20Object%20Reference) (StopEffects :type Boolean))
  (Variables|/Game/MIGRATED/Core/Character/BP_BaseCharacter.BP_BaseCharacter_C|SetCurrentHealth PlayerCharacter (Math|Float|Clamp(Float) (+ (Variables|/Game/MIGRATED/Core/Character/BP_BaseCharacter.BP_BaseCharacter_C|GetCurrentHealth PlayerCharacter) (Variables|Default|GetHealHP)) 0.0 (Variables|/Game/MIGRATED/Core/Character/BP_BaseCharacter.BP_BaseCharacter_C|GetMaxHealth PlayerCharacter)))
  (|CallParentFunction PlayerCharacter "0, 0, 0" "0, 0, 0" (Variables|/Script/Engine.Character|GetCapsuleComponent PlayerCharacter) StopEffects))

(fn FItemEffects
  (params (SoundCue :type Audio%20Component%20Object%20Reference) (Emitter :type Particle%20System%20Object%20Reference) (EmitterLoc :type Vector :default "0, 0, 0") (EmitterScale :type Vector :default "0, 0, 0") (EmitterRotation :type Rotator :default "0, 0, 0") (AttachToComponent :type Scene%20Component%20Object%20Reference))
  (|CallParentFunction SoundCue Emitter EmitterLoc EmitterScale EmitterRotation AttachToComponent))

(fn FEffectsStop
  (|CallParentFunction))

(fn FDestroyActor)