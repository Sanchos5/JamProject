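; Mana potion pickup that refills reserve ammo for the player's fire staff and electro knife.
; The AddAmmo event runs the FPickUpItem override, which skips the parent version and casts each weapon child actor in sequence.
; Each weapon gains magazine size times ReloadMultiplier, clamped to its maximum, and calls PlayFireAnimation.
; A timer then calls fDestroyActor, whose body is empty here.
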(event Custom|AddAmmo
  (params (PlayerCharacter :type %20Object%20Reference))
  (CallFunction|FPickUpItem PlayerCharacter "0, 0, 0" "0, 0, 0" 0 false))

(fn ConstructionScript
  (|CallParentFunction))

(fn FPickUpItem
  (params (PlayerCharacter :type %20Object%20Reference) (EmitterLoc :type Vector :default "0, 0, 0") (EmitterRotation :type Rotator :default "0, 0, 0") (AttachToComponent :type Scene%20Component%20Object%20Reference) (StopEffects :type Boolean))
  (Utilities|FlowControl|Sequence
    (:then_0
      (bind _asbp_ebfire_staff (Utilities|Casting|CastTo (Variables|/Script/Engine.ChildActorComponent|GetChildActor (Variables|Default|Getstaff%20actor PlayerCharacter))))
      (bind _ammoinposession (CallFunction|GetAmmo _asbp_ebfire_staff))
      ;[1 1 1] potion grants reloadmultiplier*weaponammomag amount of ammo
      (bind _output_get (Variables|Default|SetAmmoToReload (Math|Float|Truncate (* (Variables|Default|GetMagSize%20FireStaff _asbp_ebfire_staff) (Variables|Default|GetReloadMultiplier)))))
      (Variables|Default|SetAmmoInPosession _asbp_ebfire_staff (Math|Integer|Clamp(Integer) (+ _ammoinposession _output_get) 0 (Variables|Default|GetMaxAmmo%20FireStaff _asbp_ebfire_staff)))
      (CallFunction|PlayFireAnimation _asbp_ebfire_staff))
    (:then_1
      (bind _asbp_ebknife (Utilities|Casting|CastTo (Variables|/Script/Engine.ChildActorComponent|GetChildActor (Variables|Default|Getknife%20actor PlayerCharacter))))
      (bind _ammoinposession_2 (CallFunction|GetAmmo _asbp_ebknife))
      (bind _output_get_2 (Variables|Default|SetAmmoToReload (Math|Float|Truncate (* (Variables|Default|GetMagsizeElectroKnife _asbp_ebknife) (Variables|Default|GetReloadMultiplier)))))
      (Variables|Default|SetAmmoInPosession _asbp_ebknife (Math|Integer|Clamp(Integer) (+ _ammoinposession_2 _output_get_2) 0 (Variables|Default|GetMaxAmmoElectroKnife _asbp_ebknife)))
      (CallFunction|PlayFireAnimation _asbp_ebknife)))
  (Utilities|Time|SetTimerbyFunctionName 0 "fDestroyActor" (Variables|Default|GetTimer)))

(fn FDestroyActor)