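; Base Blueprint for AI enemies, with health, death and healthbar functionality, though most of its event logic is disconnected.
; BeginPlay, Tick and DisableMovement are empty, while the health, death and health-ratio overrides only forward to the parent.
; Unwired chains hold hit montage and stun, player targeting, a timed player-facing healthbar, and death with a random coin drop.
; A note says healthbar setup fails for child classes and is done in each one.
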(event Custom|DisableMovement
  (params (Delay :type Float%20%28double-precision%29)))

(event EventBeginPlay
  ;[1 1 1] event BeginPlay
)

(event EventTick
  (params (DeltaSeconds :type Float%20%28single-precision%29))
  ;[1 1 1] Healthbar Visibility and TurnToPlayer
)

(fn ConstructionScript)

(fn FGetHP
  (params (ActorHealth :type Float%20%28double-precision%29) (DamageReceived :type Float%20%28double-precision%29))
  (bind (_currenthealth _bisdead) (|CallParentFunction ActorHealth DamageReceived))
  (return _currenthealth _bisdead))

(fn FDeath
  (params (bIsDead :type Boolean) (ActorMesh :type Skeletal%20Mesh%20Component%20Object%20Reference) (DeathMontage :type Anim%20Montage%20Object%20Reference))
  (|CallParentFunction bIsDead ActorMesh DeathMontage))

(fn FGetHealthRatio
  (bind _healthratio (|CallParentFunction))
  (return _healthratio))

(fn FDisableMovement)