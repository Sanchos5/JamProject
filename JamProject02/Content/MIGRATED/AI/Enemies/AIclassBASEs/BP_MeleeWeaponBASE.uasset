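; Base Blueprint for enemy AI melee weapons, with a hitbox, an owner reference and an attack sound.
; Only BeginPlay does anything, muting the attack sound, as both hitbox overlap events are empty.
; Disconnected logic would apply point damage once per overlap from a living enemy owner to non-enemies, play the sound and reset on overlap end.
; This damage logic and the debug prints never run.
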(event OnComponentBeginOverlap(WeaponHitbox)
  (params (OverlappedComponent :type Primitive%20Component%20Object%20Reference) (OtherActor :type Actor%20Object%20Reference) (OtherComp :type Primitive%20Component%20Object%20Reference) (OtherBodyIndex :type Integer) (bFromSweep :type Boolean) (SweepResult :type Hit%20Result%20Structure%20%28by%20ref%29))
  ;[1 1 1] apply damage on hitbox overlap
)

(event OnComponentEndOverlap(WeaponHitbox)
  (params (OverlappedComponent :type Primitive%20Component%20Object%20Reference) (OtherActor :type Actor%20Object%20Reference) (OtherComp :type Primitive%20Component%20Object%20Reference) (OtherBodyIndex :type Integer))
  ;[1 1 1] apply damage on hitbox overlap
  ;;[1 1 1] reset apply damage on end component overlap
)

(event EventBeginPlay
  (Audio|Components|Audio|SetVolumeMultiplier (Variables|Default|GetAttackCue) 0.0 :!class /Script/Engine.AudioComponent))

(fn ConstructionScript)