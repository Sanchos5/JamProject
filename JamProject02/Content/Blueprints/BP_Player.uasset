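; BP_Player is a player actor that auto-attacks with a saber on a repeating half-second timer.
; BeginPlay starts the timer and attaches the Saber to the mesh's weapon socket.
; Each Damage event plays the attack montage, sphere-traces ahead and applies PlayerDamage if the hit actor has a health component.
; An unconnected branch that would enlarge the Saber never runs, and Tick is empty.
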(event Custom|Damage
  (bind _returnvalue (Transformation|GetActorLocation))
  (Animation|Montage|MontagePlay (Components|SkeletalMesh|GetAnimInstance (Variables|Character|GetMesh)) "/Game/Characters/Shrekich/Shrek/Animations/AM_AttackMontage.AM_AttackMontage" 1.0 "MontageLength" 0.0 true)
  (bind _outhit (Collision|SphereTraceByChannel _returnvalue (+ _returnvalue (* (Transformation|GetActorForwardVector) 2.2e+02)) 9e+01 "TraceTypeQuery1" false 0 "None"))
  (Utilities|IsValid (Class|HealthComponent|FindHealthComponent (.HitActor (Collision|BreakHitResult _outhit)))
    (:Is%20Valid
      (Game|Damage|ApplyDamage (.HitActor (Collision|BreakHitResult _outhit)) (Variables|Default|GetPlayerDamage) 0 self))))

(event EventBeginPlay
  (bind _returnvalue (Utilities|Time|SetTimerbyEvent (delegate Custom|Damage) 0.5 true))
  (Variables|Default|SetNewVar _returnvalue)
  (Transformation|AttachComponentToComponent (Variables|Default|GetSaber) (Variables|Character|GetMesh) "Weapon_socket" "KeepRelative" "KeepRelative" "KeepRelative" true))

(event EventTick
  (params (DeltaSeconds :type Float%20%28single-precision%29)))

(fn ConstructionScript)