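; BP_Laser is a short-lived enemy laser beam actor that turns to follow the player and deals damage at its far end.
; A looping timer retargets yaw toward the player and plays the laser sound, while Tick rotates at constant speed and stretches the cylinder to the clamped player distance.
; A second timer applies radial damage near the beam's end; its capsule trace result is unused.
; The actor destroys itself after a fixed delay.
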(event Custom|Damage
  (bind _returnvalue (Transformation|GetActorLocation))
  (bind _returnvalue_2 (Transformation|GetActorForwardVector))
  (bind _transform (Variables|Default|GetTransform))
  (bind _returnvalue_3 (* _returnvalue_2 _transform))
  (bind _returnvalue_4 (+ _returnvalue _returnvalue_3))
  ;[1 1 1] Laser Damage
  (Variables|Default|SetEndPoint (Math|Vector|MakeVector (.x _returnvalue_4) (.y _returnvalue_4) (.z _returnvalue_4)))
  (Collision|CapsuleTraceByChannel _returnvalue (Math|Vector|MakeVector (- (.x (Variables|Default|GetEndPoint)) 5e+01) (- (.y (Variables|Default|GetEndPoint)) 5e+01) (- (.z (Variables|Default|GetEndPoint)) 8e+01)) (Variables|Default|GetDamageRadius) 5e+01 "TraceTypeQuery1" false 0 "None" true "(R=1.000000,G=0.000000,B=0.000000,A=0.000000)" "(R=0.000000,G=1.000000,B=0.000000,A=1.000000)" 1.0)
  (Game|Damage|ApplyRadialDamage (Variables|Default|GetNDamage) (Math|Vector|MakeVector (.x (Variables|Default|GetEndPoint)) (.y (Variables|Default|GetEndPoint)) (- (.z (Variables|Default|GetEndPoint)) 8e+01)) (Variables|Default|GetDamageRadius) 0 0 0 0 true "ECC_Visibility"))

(event Custom|Adjust%20Location
  ;[1 1 1] calculate laser transform
  (Variables|Default|SetTargetRotation (Math|Rotator|MakeRotator 0.0 0.0 (.yaw (Math|Rotator|FindLookatRotation (Transformation|GetActorLocation self) (Transformation|GetWorldLocation (Variables|/Script/Engine.Character|GetMesh (Variables|Default|GetPlayerRef)))))))
  (Audio|SpawnSound2D "/Game/Blueprints/AI/Enemy/Laser/A_Laser.A_Laser" 0.5 1.0 0.0 0))

(event Collision|EventActorBeginOverlap
  (params (OtherActor :type Actor%20Object%20Reference)))

(event EventBeginPlay
  (bind _asbp_player (Utilities|Casting|CastToBP_Player (Game|Player|GetPlayerPawn 0)))
  (Variables|Default|SetPlayerRef _asbp_player)
  (Utilities|FlowControl|Sequence
    (:then_0
      ;[1 1 1] timers
      (Utilities|Time|SetTimerbyEvent (delegate Custom|Adjust%20Location) (Variables|Default|GetRotationTimer) true)
      (CallFunction|AdjustLocation)
      (Utilities|Time|SetTimerbyEvent (delegate Custom|Damage) (Variables|Default|GetDamageTimer) true))
    (:then_1
      (Utilities|FlowControl|Delay 12.0)
      (Actor|DestroyActor))))

(event EventTick
  (params (DeltaSeconds :type Float%20%28single-precision%29))
  (bind _cylinder (Variables|Default|GetCylinder))
  (Utilities|FlowControl|Sequence
    (:then_0
      ;[1 1 1] transform and rotate laser to track player
      (bind _output_get (Variables|Default|SetTransform (Math|Float|Clamp(Float) (Math|Vector|Distance(Vector) (Transformation|GetActorLocation self) (Transformation|GetWorldLocation (Variables|/Script/Engine.Character|GetMesh (Variables|Default|GetPlayerRef)))) 0.0 8e+02)))
      (Transformation|SetWorldScale3D _cylinder (Math|Vector|MakeVector 0.1 0.1 (/ _output_get 1e+02)))
      (Transformation|SetRelativeLocation _cylinder (Math|Vector|MakeVector (/ _output_get 2.0) 0.0 0.0) false false))
    (:then_1
      (Transformation|SetWorldRotation (Variables|Default|GetDefaultSceneRoot) (Class|KismetMathLibrary|RInterptoConstant (Transformation|GetWorldRotation (Variables|Default|GetDefaultSceneRoot)) (Variables|Default|GetTargetRotation) DeltaSeconds 5e+01) false false))))

(fn ConstructionScript)