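; Ranged enemy Blueprint that provides a hitscan-style distance attack against the player.
; The Distanceattack event sphere-traces forward from the actor on the Visibility channel, with timed debug drawing, and applies fixed damage if the hit actor is BP_Player.
; Nothing in this file triggers the attack, and the default BeginPlay, overlap and Tick events are disabled stubs.
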(event Custom|Distance%20attack
  (bind _returnvalue (Transformation|GetActorLocation))
  (bind _outhit (Collision|SphereTraceByChannel _returnvalue (+ _returnvalue (* (Transformation|GetActorForwardVector) 1e+03)) 3e+01 "TraceTypeQuery1" false 0 "ForDuration"))
  (bind _asbp_player (Utilities|Casting|CastToBP_Player (.HitActor (Collision|BreakHitResult _outhit))))
  (Game|Damage|ApplyDamage _asbp_player 5e+01 0 self))

(event EventBeginPlay
  (|CallParentFunction) ; This node is disabled and will not be called.\nDrag off pins to build functionality.
)

(event Collision|EventActorBeginOverlap
  (params (OtherActor :type Actor%20Object%20Reference))
  (|CallParentFunction OtherActor) ; This node is disabled and will not be called.\nDrag off pins to build functionality.
)

(event EventTick
  (params (DeltaSeconds :type Float%20%28single-precision%29))
  (|CallParentFunction DeltaSeconds) ; This node is disabled and will not be called.\nDrag off pins to build functionality.
)

(fn ConstructionScript
  (|CallParentFunction))