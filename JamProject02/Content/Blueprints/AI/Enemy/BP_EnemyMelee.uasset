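; Melee enemy Blueprint that attaches a skeletal mesh to its RightHand socket and runs debug-drawn hit traces for attacks.
; MeleeRaycast starts a fast looping timer that capsule-traces between the mesh's LineTraceStart and LineTraceEnd sockets, clearing it after the given delay.
; The hit handling is unfinished: the health-component check leads nowhere, and setting HitActor and applying SwordDamage are unwired, leaving only debug prints.
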(event Custom|MeleeRaycast
  (params (Delay :type Float%20%28double-precision%29))
  (bind _hit_actor (Variables|Default|GetHit%20Actor))
  (bind _returnvalue (Utilities|Time|SetTimerbyEvent (delegate Custom|CustomEvent) 0.01 true))
  (Utilities|FlowControl|Delay Delay)
  (Utilities|Time|ClearandInvalidateTimerbyHandle _returnvalue)
  (Utilities|IsValid _hit_actor
    (:Is%20Valid
      (Development|PrintString (Utilities|String|BuildString(Object) "" "MELEE APPLY DAMAGE: " _hit_actor " ") true true "(R=1.000000,G=0.033202,B=0.000000,A=1.000000)" 5.0))))

(event Custom|CustomEvent
  (bind _skeletalmesh (Variables|Default|GetSkeletalMesh))
  (bind _outhit (Collision|CapsuleTraceByChannel (Transformation|GetSocketLocation _skeletalmesh "LineTraceStart") (Transformation|GetSocketLocation _skeletalmesh "LineTraceEnd") 3e+01 3e+01 "TraceTypeQuery1" false 0 "ForDuration" true "(R=1.000000,G=0.000000,B=0.000000,A=1.000000)" "(R=0.000000,G=1.000000,B=0.000000,A=1.000000)" (stale Custom|MeleeRaycast Delay)))
  (Utilities|IsValid (Class|HealthComponent|FindHealthComponent (.HitActor (Collision|BreakHitResult _outhit)))))

(event EventBeginPlay
  (Development|PrintString (Utilities|String|BuildString(Object) "" "" (Pawn|GetController)) true true "(R=0.000000,G=1.000000,B=0.063842,A=1.000000)" 1e+01)
  (Transformation|AttachComponentToComponent (Variables|Default|GetSkeletalMesh) (Variables|Character|GetMesh) "RightHand" "KeepRelative" "KeepRelative" "KeepRelative" true))

(event Collision|EventActorBeginOverlap
  (params (OtherActor :type Actor%20Object%20Reference))
  (|CallParentFunction OtherActor) ; This node is disabled and will not be called.\nDrag off pins to build functionality.
)

(event EventTick
  (params (DeltaSeconds :type Float%20%28single-precision%29))
  (|CallParentFunction DeltaSeconds) ; This node is disabled and will not be called.\nDrag off pins to build functionality.
)

(fn ConstructionScript
  (|CallParentFunction))