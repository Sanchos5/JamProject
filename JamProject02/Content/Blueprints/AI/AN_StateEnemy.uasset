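; Anim notify state for enemy melee attack animations that deals the enemy's hit damage to the player.
; When the notify window begins, it casts the mesh owner to BP_EnemyCharacter and measures its distance to player 0.
; If within AttackDistanceMelee, it applies DamagePerHit once, with no trace or overlap check.
; The end event only performs the cast, and the debug prints are disconnected.
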(fn ReceivedNotifyBegin
  (params (MeshComp :type Skeletal%20Mesh%20Component%20Object%20Reference) (Animation :type Anim%20Sequence%20Base%20Object%20Reference) (TotalDuration :type Float%20%28single-precision%29) (EventReference :type Anim%20Notify%20Event%20Reference%20Structure%20%28by%20ref%29))
  (bind _returnvalue (Components|GetOwner MeshComp))
  (bind _returnvalue_2 (Game|GetPlayerCharacter _returnvalue))
  (bind _asbp_enemy_character (Utilities|Casting|CastToBP_EnemyCharacter _returnvalue))
  (if (<= (Math|Vector|Distance(Vector) (Transformation|GetActorLocation _returnvalue) (Transformation|GetActorLocation _returnvalue_2)) (Variables|/Game/Blueprints/AI/Enemy/BP_EnemyCharacter.BP_EnemyCharacter_C|GetAttackDistanceMelee _asbp_enemy_character))
    (bind _returnvalue_3 (Game|Damage|ApplyDamage _returnvalue_2 (Variables|/Game/Blueprints/AI/Enemy/BP_EnemyCharacter.BP_EnemyCharacter_C|GetDamage%20Per%20Hit _asbp_enemy_character) 0 _asbp_enemy_character))
    (return true)))

(fn ReceivedNotifyEnd
  (params (MeshComp :type Skeletal%20Mesh%20Component%20Object%20Reference) (Animation :type Anim%20Sequence%20Base%20Object%20Reference) (EventReference :type Anim%20Notify%20Event%20Reference%20Structure%20%28by%20ref%29))
  (Utilities|Casting|CastToBP_EnemyCharacter (Components|GetOwner MeshComp)))