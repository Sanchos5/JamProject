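; BP_Book_stacking is a construction-time placement tool in the Abandoned Library book assets that builds a grid of copies of one static mesh, presumably stacked books.
; The Construction Script loops over rows and columns, adding a separate static mesh component per cell, spaced along local X by row and Z by column.
; The X spacing is truncated to a whole number.
; The event graph holds no active logic.
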(event EventBeginPlay)

(event Collision|EventActorBeginOverlap
  (params (OtherActor :type Actor%20Object%20Reference)))

(event EventTick
  (params (DeltaSeconds :type Float%20%28single-precision%29)))

(fn ConstructionScript
  (for _index (range 0 (- (Variables|Default|GetNumber_of_rows) 1))
    (for _index_2 (range 0 (- (Variables|Default|GetNumber_Of_Columns) 1))
      (bind _returnvalue (AddComponent|AddStaticMeshComponent false (Math|Transform|MakeTransform (Math|Vector|MakeVector (Math|Conversions|ToFloat(Integer) (* _index (Math|Float|Truncate (Variables|Default|GetOffset_X_pos)))) 0.0 (Math|Conversions|ToFloat(Integer) (* _index_2 (Variables|Default|Getoffset_z)))) "0, 0, 0" "1.000000,1.000000,1.000000")))
      (Components|StaticMesh|SetStaticMesh _returnvalue (Variables|Default|GetStatic_mesh)))))