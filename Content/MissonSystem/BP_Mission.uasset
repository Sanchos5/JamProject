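; BP_Mission is an actor representing a single mission in the mission system, holding its info, owning player character, state and phase.
; Init stores the mission info and owner and resets the phase to zero.
; UpdateState and UpdatePhase print a debug message, store the new value, then broadcast a change dispatcher that passes the mission itself and that value.
; The event graph and construction script are empty.
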(event EventBeginPlay)

(event Collision|EventActorBeginOverlap
  (params (OtherActor :type Actor%20Object%20Reference)))

(event EventTick
  (params (DeltaSeconds :type Float%20%28single-precision%29)))

(fn ConstructionScript)

(fn Init
  (params (InMissionInfo :type Mission%20Info%20Struct%20Structure) (InPlayerCharacter :type BP%20FPS%20Character%20Object%20Reference))
  (Variables|Default|SetInfo InMissionInfo)
  (Variables|Default|SetOwnerPlayerCharacter InPlayerCharacter)
  (Variables|Default|SetPhase 0))

(fn UpdateState
  (params (InNewState :type MissionState_Enum%20Enum :default "NewEnumerator0"))
  (Development|PrintString (Utilities|String|Append (Utilities|String|ToString(Text) (.nameui (Variables|Default|GetInfo))) "" "Changed State to '" (Utilities|String|ToString(Byte) InNewState) "'"))
  (bind _output_get (Variables|Default|SetState InNewState))
  (Default|CallOnChangedStateMission self _output_get))

(fn UpdatePhase
  (params (InNewPhase :type Integer))
  (Development|PrintString (Utilities|String|Append "" (Utilities|String|ToString(Text) (.nameui (Variables|Default|GetInfo))) "Changed phase to '" (Utilities|String|ToString(Integer) InNewPhase) "'"))
  (bind _output_get (Variables|Default|SetPhase InNewPhase))
  (Default|CallOnChangedPhaseMission self _output_get))