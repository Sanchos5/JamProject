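; Mission manager that keeps a list of missions and tracks which one is current.
; Added missions are queued, and the first becomes current if none is; switching updates both missions' states, moves the state-change binding and broadcasts the change.
; When the current mission reaches its final state, it is removed and the first remaining mission takes over.
; Helpers find a mission by name, remove one or clear all.
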(event Custom|OnChangedStateMission
  (params (InMission :type BP%20Mission%20Object%20Reference) (InNewState :type MissionState_Enum%20Enum :default "NewEnumerator0"))
  (bind _missions (Variables|Default|GetMissions))
  (if (Utilities|Enum|Equal(Enum) InNewState "NewEnumerator2")
    (CallFunction|RemoveMissionbyPointer InMission)
    (if (Utilities|Array|IsNotEmpty _missions)
      (CallFunction|SetCurrentMission (Utilities|Array|Get(acopy) _missions)))))

(event EventBeginPlay)

(event Collision|EventActorBeginOverlap
  (params (OtherActor :type Actor%20Object%20Reference)))

(event EventTick
  (params (DeltaSeconds :type Float%20%28single-precision%29)))

(fn ConstructionScript)

(fn AddNextMission
  (params (InMission :type BP%20Mission%20Object%20Reference))
  (Utilities|Array|Add (Variables|Default|GetMissions) InMission)
  (Default|UpdateState InMission "NewEnumerator1")
  (Utilities|IsValid (Variables|Default|GetCurrrentMission)
    (:Is%20Not%20Valid
      (CallFunction|SetCurrentMission InMission))))

(fn SetCurrentMission
  (params (InMission :type BP%20Mission%20Object%20Reference))
  (if (!= InMission (Variables|Default|GetCurrrentMission))
    (Utilities|IsValid (Variables|Default|GetCurrrentMission)
      (:Is%20Valid
        (EventDispatchers|UnbindEventfromOnChangedStateMission (Variables|Default|GetCurrrentMission) (EventDispatchers|CreateEvent :!event Custom|OnChangedStateMission))
        (if (Utilities|Enum|NotEqual(Enum) (Variables|/Game/MissonSystem/BP_Mission.BP_Mission_C|GetState (Variables|Default|GetCurrrentMission)) "NewEnumerator2")
          (Default|UpdateState (Variables|Default|GetCurrrentMission) "NewEnumerator1"))
        (Variables|Default|SetCurrrentMission 0))
      (:Is%20Not%20Valid
        _))
    (Utilities|IsValid InMission
      (:Is%20Valid
        (bind _output_get (Variables|Default|SetCurrrentMission InMission))
        (Default|UpdateState _output_get "NewEnumerator0")
        (EventDispatchers|BindEventtoOnChangedStateMission _output_get (EventDispatchers|CreateEvent :!event Custom|OnChangedStateMission)))
      (:Is%20Not%20Valid
        _))
    (Default|CallOnChangedCurrentMission (Variables|Default|GetCurrrentMission))))

(fn RemoveAllMissions
  (CallFunction|SetCurrentMission)
  (Utilities|Array|Clear (Variables|Default|GetMissions)))

(fn RemoveMissionbyPointer
  (params (InMission :type BP%20Mission%20Object%20Reference))
  (bind _missions (Variables|Default|GetMissions))
  (Utilities|IsValid InMission
    (:Is%20Valid
      (if (== (Variables|Default|GetCurrrentMission) InMission)
        (CallFunction|SetCurrentMission))
      (Utilities|Array|RemoveItem _missions InMission)
      (if (and (Utilities|Array|IsNotEmpty _missions) (not (Utilities|IsValid (Variables|Default|GetCurrrentMission))))
        (CallFunction|SetCurrentMission (Utilities|Array|Get(acopy) (Variables|Default|GetMissions)))))))

(fn FindMission
  (params (InName :type Name))
  (for _array_element (Variables|Default|GetMissions)
    (if (== InName (.name (Variables|/Game/MissonSystem/BP_Mission.BP_Mission_C|GetInfo _array_element)))
      (return _array_element)))
  (return 0))