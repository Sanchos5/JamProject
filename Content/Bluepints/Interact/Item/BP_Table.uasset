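; Interactive table actor that lays out letter pieces on a nine-point grid and gives the player a close-up camera view of it.
; On BeginPlay it caches grid world positions in GridStructure and spawns each BP_Letter at a random, non-repeating slot.
; PlayerSnap locks the player, hands cursor control to WBP_Interface and eases the camera to CameraSnapPoint via Tick.
; PlayerRelease restores camera, input and movement; MoveLetter is an empty stub.
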(event Custom|PlayerSnap
  (bind _returnvalue (Game|GetPlayerController 0))
  (bind _playerref (Variables|Default|GetPlayerRef))
  (bind _followcamera (Variables|/Game/Bluepints/Core/Player/BP_FPS_Character.BP_FPS_Character_C|GetFollowCamera _playerref))
  ;[1 1 1] disable player movement input
  (Variables|/Game/Bluepints/Core/Player/BP_FPS_Character.BP_FPS_Character_C|SetbCanPlayerMove (Variables|Default|GetPlayerRef) false)
  ;[1 1 1] set camera location to SnapPoint and rotation to look at the table
  ;;[1 1 1] save initial camera loc and rot to return to
  (Variables|GridSnapPositionsWorld|SetCameraRootWorldLoc (Transformation|GetWorldLocation _followcamera))
  (Variables|Default|SetCameraRootWorldRot (Transformation|GetWorldRotation _followcamera))
  ;;[1 1 1] start even tick move camera function
  (Variables|Default|SetbMoveCamera true)
  ;[1 1 1] change game mode to input game and ui disable camera input and set player snap true
  (Input|SetInputModeGameandUI _returnvalue 0 "DoNotLock" true false)
  (Variables|/Script/Engine.PlayerController|SetbShowMouseCursor _returnvalue false)
  (Variables|/Game/Bluepints/Core/Player/BP_FPS_Character.BP_FPS_Character_C|SetIsLook? (Variables|Default|GetPlayerRef) false)
  ;[1 1 1] delegate cursor controls to wbp interface
  (bind _aswbp_interface (Utilities|Casting|CastToWBP_Interface (Variables|/Game/Bluepints/Core/Player/BP_FPS_Character.BP_FPS_Character_C|GetWidgetGame (Variables|Default|GetPlayerRef))))
  (Default|CursorSnap _aswbp_interface))

(event Custom|PlayerRelease
  (bind _returnvalue (Game|GetPlayerController 0))
  (bind _playerref (Variables|Default|GetPlayerRef))
  (bind _playerref_2 (Variables|Default|GetPlayerRef))
  (bind _camerarootworldrot (Variables|Default|GetCameraRootWorldRot))
  (bind _followcamera (Variables|/Game/Bluepints/Core/Player/BP_FPS_Character.BP_FPS_Character_C|GetFollowCamera _playerref))
  ;[1 1 1] reverse widget changes
  (Default|PlayerRelease (Variables|/Game/Bluepints/Core/Player/BP_FPS_Character.BP_FPS_Character_C|GetWidgetGame (Variables|Default|GetPlayerRef)))
  ;[1 1 1] player can move camera
  (Variables|/Game/Bluepints/Core/Player/BP_FPS_Character.BP_FPS_Character_C|SetIsLook? (Variables|Default|GetPlayerRef) true)
  (Variables|/Script/Engine.PlayerController|SetbShowMouseCursor _returnvalue false)
  ;[1 1 1] return input mode to game only
  (Input|SetInputModeGameOnly _returnvalue false)
  ;[1 1 1] check if player camera needs resetting
  (if (Utilities|Operators|EqualEqual (Transformation|GetWorldLocation (Variables|/Game/Bluepints/Core/Player/BP_FPS_Character.BP_FPS_Character_C|GetFollowCamera _playerref_2)) (Transformation|GetWorldLocation (Variables|/Game/Bluepints/Core/Player/BP_FPS_Character.BP_FPS_Character_C|GetCameraRoot _playerref_2)) 1.0)
    _
    (else
      ;[1 1 1] move camera back to saved location and rotation
      (Transformation|SetWorldLocation (Variables|/Game/Bluepints/Core/Player/BP_FPS_Character.BP_FPS_Character_C|GetSpringArm _playerref) (Math|Interpolation|VInterpTo (Transformation|GetWorldLocation _followcamera) (Variables|GridSnapPositionsWorld|GetCameraRootWorldLoc) 1.0 5.0) false false)
      (Transformation|SetWorldRotation _followcamera (Math|Interpolation|RInterpTo (Transformation|GetWorldRotation _followcamera) (Math|Rotator|MakeRotator 0.0 (.pitch _camerarootworldrot) (.yaw _camerarootworldrot)) 0.5 45.0) false false)))
  ;[1 1 1] give player back movement controls
  (Variables|/Game/Bluepints/Core/Player/BP_FPS_Character.BP_FPS_Character_C|SetbCanPlayerMove (Variables|Default|GetPlayerRef) true))

(event EventTick
  (params (DeltaSeconds :type Float%20%28single-precision%29))
  ;[1 1 1] tick delta seconds
  (bind _output_get (Variables|Default|SetDelta%20Seconds DeltaSeconds))
  (CallFunction|MoveCamera _output_get))

(event EventBeginPlay
  ;[1 1 1] FPS Player Character Ref
  (bind _asbp_fps_character (Utilities|Casting|CastToBP_FPS_Character (Game|GetPlayerCharacter 0)))
  (Variables|Default|SetPlayerRef _asbp_fps_character)
  ;[1 1 1] save grid snap positions world loc to array
  (CallFunction|SetUpArrayOfWorldGridPositions)
  (CallFunction|SpawnBPLettersatGridPositions))

(fn ConstructionScript)

(fn SetUpArrayOfWorldGridPositions
  (bind _gridstructure (Variables|Default|GetGridStructure))
  (bind _output_get (Variables|GridSnapPositionsWorld|SetGridPosition1 (Transformation|GetWorldLocation (Variables|Default|GetGrid1))))
  (Utilities|Array|SetArrayElem (.location _gridstructure) 0 _output_get)
  (Utilities|Array|SetArrayElem (.location _gridstructure) 1 _output_get)
  (bind _output_get_2 (Variables|GridSnapPositionsWorld|SetGridPosition2 (Transformation|GetWorldLocation (Variables|Default|GetGrid2))))
  (Utilities|Array|SetArrayElem (.location _gridstructure) 2 _output_get_2)
  (bind _output_get_3 (Variables|GridSnapPositionsWorld|SetGridPosition3 (Transformation|GetWorldLocation (Variables|Default|GetGrid3))))
  (Utilities|Array|SetArrayElem (.location _gridstructure) 3 _output_get_3)
  (bind _output_get_4 (Variables|GridSnapPositionsWorld|SetGridPosition4 (Transformation|GetWorldLocation (Variables|Default|GetGrid4))))
  (Utilities|Array|SetArrayElem (.location _gridstructure) 4 _output_get_4)
  (bind _output_get_5 (Variables|GridSnapPositionsWorld|SetGridPosition5 (Transformation|GetWorldLocation (Variables|Default|GetGrid5))))
  (Utilities|Array|SetArrayElem (.location _gridstructure) 5 _output_get_5)
  (bind _output_get_6 (Variables|GridSnapPositionsWorld|SetGridPosition6 (Transformation|GetWorldLocation (Variables|Default|GetGrid6))))
  (Utilities|Array|SetArrayElem (.location _gridstructure) 6 _output_get_6)
  (bind _output_get_7 (Variables|GridSnapPositionsWorld|SetGridPosition7 (Transformation|GetWorldLocation (Variables|Default|GetGrid7))))
  (Utilities|Array|SetArrayElem (.location _gridstructure) 7 _output_get_7)
  (bind _output_get_8 (Variables|GridSnapPositionsWorld|SetGridPosition8 (Transformation|GetWorldLocation (Variables|Default|GetGrid8))))
  (Utilities|Array|SetArrayElem (.location _gridstructure) 8 _output_get_8)
  (bind _output_get_9 (Variables|GridSnapPositionsWorld|SetGridPosition9 (Transformation|GetWorldLocation (Variables|Default|GetGrid9))))
  (Utilities|Array|SetArrayElem (.location _gridstructure) 9 _output_get_9)
  (return))

(fn SpawnBPLettersatGridPositions
  (bind _gridstructure (Variables|Default|GetGridStructure))
  (for _array_element (Variables|Default|GetBPLetters1To7)
    ;[1 1 1] choose a random grid point location index Except 0
    (bind _output_get (Variables|Default|SetRandomUnrepeatedIntInRange (Utilities|Array|Get(acopy) (Variables|Default|GetGridLocationsIntRange) (Math|Random|RandomIntegerinRange 1 (Variables|Default|GetRandonUnrepeatedIntMax))) :!label _label))
    (if (== _output_get 0)
      (goto _label)
      (else
        ;[1 1 1] spawn bp letter at a chosen random location
        (bind _returnvalue (Game|SpawnActorfromClass _array_element (Math|Transform|MakeTransform (Utilities|Array|Get(acopy) (.location (Variables|Default|GetGridStructure)) _output_get) "0.000000,-90.000000,0.000000" "1.000000,1.000000,1.000000") "AdjustIfPossibleButAlwaysSpawn" "MultiplyWithRoot" 0 0))
        ;[1 1 1] set letter starter position
        (bind _asbp_letter (Utilities|Casting|CastToBP_Letter _returnvalue))
        (Variables|/Game/Bluepints/Items/FamilyPhoto/BP_Letter.BP_Letter_C|SetNewPosition _asbp_letter (Utilities|Array|Get(acopy) (.location (Variables|Default|GetGridStructure)) _output_get))
        ;[1 1 1] save positions to struct
        (Utilities|Array|SetArrayElem (.letter _gridstructure) _output_get _returnvalue)
        (Utilities|Array|SetArrayElem (.letteringrid _gridstructure) _output_get true)
        ;[1 1 1] remove chosen index from the range of indexes so spawn locations don't repeat
        (Utilities|Array|RemoveItem (Variables|Default|GetGridLocationsIntRange) (Variables|Default|GetRandomUnrepeatedIntInRange))
        (Math|Integer|DecrementInt (Variables|Default|GetRandonUnrepeatedIntMax))))))

(fn MoveCamera
  (params (DeltaTime :type Float%20%28single-precision%29))
  (bind _camerasnappoint (Variables|Default|GetCameraSnapPoint))
  (bind _playerref (Variables|Default|GetPlayerRef))
  (bind _returnvalue (Transformation|GetWorldLocation _camerasnappoint))
  (bind _followcamera (Variables|/Game/Bluepints/Core/Player/BP_FPS_Character.BP_FPS_Character_C|GetFollowCamera _playerref))
  (if (Variables|Default|GetbMoveCamera)
    ;[1 1 1] set camera location to snap point and rotation to look at the table
    (bind _output_get (LocalVariables|SetLookAtRot (Math|Rotator|FindLookatRotation _returnvalue (Transformation|GetWorldLocation (Variables|Default|GetDefaultSceneRoot)))))
    (Transformation|SetWorldLocationAndRotation _followcamera (Math|Interpolation|VInterpTo (Transformation|GetWorldLocation _followcamera) _returnvalue DeltaTime 5.0) (Math|Interpolation|RInterpTo (Transformation|GetWorldRotation _followcamera) _output_get DeltaTime 45.0) false false)
    ;[1 1 1] stop when target location and rotation reached
    (if (and (Utilities|Operators|EqualEqual (Transformation|GetWorldLocation _followcamera) (Transformation|GetWorldLocation (Variables|Default|GetCameraSnapPoint)) 3.0) (Utilities|Operators|EqualEqual (Transformation|GetWorldRotation _followcamera) (LocalVariables|GetLookAtRot) 3.0))
      (Variables|Default|SetbMoveCamera false))))

(fn GetButtonGridLocations
  (bind _gridstructure (Variables|Default|GetGridStructure))
  (Development|PrintString "Send vectors: " true true "(R=0.000000,G=0.660000,B=1.000000,A=1.000000)" 3e+01)
  (for (_array_element _array_index) (.location _gridstructure)
    (Development|PrintString "Hello" true true "(R=1.000000,G=0.788955,B=0.000000,A=1.000000)" 3e+01))
  (return (.location _gridstructure)))

(fn MoveLetter
  (params (NewLocation :type Vector :default "0, 0, 0"))
  (return))