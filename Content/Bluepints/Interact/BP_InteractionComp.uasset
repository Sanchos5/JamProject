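; BP_InteractionComp is an interaction component that detects interactable actors in front of the player's camera.
; TraceInteract runs a Visibility line trace from the player's FollowCamera along its forward vector for InteractDistance.
; Interact uses that hit: for actors implementing BPI_Interaction, it turns on the Target's interact text and immediately calls InteractWithMessage, otherwise it turns the text off.
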(event EventBeginPlay)

(event EventTick
  (params (DeltaSeconds :type Float%20%28single-precision%29)))

(fn TraceInteract
  (bind _asbp_player (CallFunction|FindPlayerCast))
  (bind _followcamera (Variables|/Game/Bluepints/BP_Player.BP_Player_C|GetFollowCamera _asbp_player))
  (bind _returnvalue (Transformation|GetWorldLocation _followcamera))
  (Utilities|IsValid _asbp_player
    (:Is%20Valid
      (bind (_outhit _returnvalue_2) (Collision|LineTraceByChannel _returnvalue (+ _returnvalue (* (Math|Vector|GetForwardVector _followcamera) (Variables|Default|GetInteractDistance))) "TraceTypeQuery1" false 0 "None"))
      (return _outhit _returnvalue_2))))

(fn Interact
  (params (Target :type WBP%20Interface%20Object%20Reference))
  (bind (_outhit _returnvalue) (CallFunction|TraceInteract))
  (if _returnvalue
    (bind _output_get (Variables|Default|SetHit%20Actor (.HitActor (Collision|BreakHitResult _outhit))))
    (if (Utilities|DoesObjectImplementInterface (Variables|Default|GetHit%20Actor) "/Game/Bluepints/Interact/BPI_Interaction.BPI_Interaction_C")
      (Default|WInteractText Target true)
      (Class|BPIInteraction|Interactwith(Message) _output_get)
      (else
        (Default|WInteractText Target false :!label _label)))
    (else
      (Variables|Default|SetHit%20Actor 0)
      (goto _label))))