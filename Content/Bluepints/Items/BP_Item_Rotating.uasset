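; BP_Item_Rotating is an item Blueprint whose static mesh turns in yaw when its Rotate event fires.
; Rotate confirms the player is BP_FPS_Character, prints a debug string, then applies one interpolation step toward 90 degrees past the current yaw.
; Item getters report no fracture and the first item-type enum entry, while Get Mesh returns nothing.
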(event Custom|Rotate
  (bind _sm (Variables|Default|GetSM))
  (bind _returnvalue (Transformation|GetWorldRotation _sm))
  (Utilities|Casting|CastToBP_FPS_Character (Game|GetPlayerCharacter 0))
  (Development|PrintString "BP FPS Successfull")
  (Transformation|SetWorldRotation _sm (Math|Interpolation|RInterpTo (Math|Rotator|MakeRotator 0.0 0.0 (.yaw _returnvalue)) (Math|Rotator|MakeRotator 0.0 0.0 (+ (.yaw _returnvalue) 9e+01)) (Utilities|Time|GetWorldDeltaSeconds) 0.0) false false))

(fn ConstructionScript
  (|CallParentFunction))

(fn GetFractureBool
  (return false))

(fn GetItemType
  (return "NewEnumerator0"))

(fn GetMesh
  (return 0))