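; BP_Input_Slot is an input that switches on when an accepted item is placed in its trigger volume.
; On overlap it checks that the item is unfractured, interactable, of an accepted class and matches the slot index, and that the slot is off.
; A DoOnce-gated sequence drops the item, slots it to the trigger, turns the state on and disables item collision.
; UnSlotItem turns the state off and resets the gate.
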(event OnComponentBeginOverlap(TriggerVolume)
  (params (OverlappedComponent :type Primitive%20Component%20Object%20Reference) (OtherActor :type Actor%20Object%20Reference) (OtherComp :type Primitive%20Component%20Object%20Reference) (OtherBodyIndex :type Integer) (bFromSweep :type Boolean) (SweepResult :type Hit%20Result%20Structure%20%28by%20ref%29))
  (Utilities|CanSlotItem? OtherActor
    (:true
      (bind _index (Class|BPIInteraction|GetDropItemIndex(Message) OtherActor))
      (if (== (Variables|Default|GetIndexSlot) _index)
        (Utilities|FlowControl|DoOnce false
          (:Completed
            (Class|BPIInteraction|DropItem(Message) OtherActor "0, 0, 0" false)
            (Class|BPIInteraction|SlotItem(Message) OtherActor (Variables|Default|GetTrigger%20Volume))
            (CallFunction|SetStateon)
            (Collision|SetActorEnableCollision OtherActor false)))))))

(event EventUnSlotItem
  (CallFunction|SetStateOff)
  (Utilities|FlowControl|DoOnce false) ; enters at Reset
)

(fn ConstructionScript)

(fn GetMesh
  (return 0))

(fn GetInteractionType
  (return))

(fn GetPickupItem
  (return false))

(fn GetDropItemIndex
  (return (Variables|Default|GetIndexSlot)))