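; Puzzle slot actor that detects placed shapes and spawns BP_PiramidaDown once the puzzle counts as solved.
; The trigger volume matches tags BP1–BP4 against their InIndexCube flags and increments IndexSlot on a match.
; Any actor overlap separately runs SummIndex, which requires IdexSumReqCurrent to equal four, a counter raised only by IndexSumReq, never called here.
; Work in progress: debug prints report results, and several helper functions are stubs.
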(event OnComponentBeginOverlap(TriggerVolume)
  (params (OverlappedComponent :type Primitive%20Component%20Object%20Reference) (OtherActor :type Actor%20Object%20Reference) (OtherComp :type Primitive%20Component%20Object%20Reference) (OtherBodyIndex :type Integer) (bFromSweep :type Boolean) (SweepResult :type Hit%20Result%20Structure%20%28by%20ref%29))
  ;[1 1 1] Я в душе не ебу как это реализовать
  (if (and (Actor|ActorHasTag OtherActor "BP1") (Variables|Default|GetInIndexCube))
    (Development|PrintString "Да Has Tag BP1")
    (if true :!label _label
      (bind _result (Math|Integer|IncrementInt (Variables|Default|GetIndexSlot))
        (:%20%20
          (bind _output_get (Variables|Default|SetIndexSlot _result))
          (Development|PrintString (Utilities|String|Append "Было" (Utilities|String|ToString(Integer) (Variables|Default|GetIndexSlot)) "Стало" (Utilities|String|ToString(Integer) _output_get))))))
    (elif (and (Actor|ActorHasTag OtherActor "BP2") (Variables|Default|GetInIndexCube2))
      (Development|PrintString "Да Has Tag BP2")
      (goto _label)
      (elif (and (Actor|ActorHasTag OtherActor "BP3") (Variables|Default|GetInIndexCube3))
        (Development|PrintString "Да Has Tag BP3")
        (goto _label)
        (elif (and (Actor|ActorHasTag OtherActor "BP4") (Variables|Default|GetInIndexCube4))
          (Development|PrintString "Да Has Tag BP4")
          (goto _label))))))

(event Custom|SummIndex
  (if (== (Variables|Default|GetIdexSumReqCurrent) 4)
    (Game|SpawnActorfromClass "/Game/Bluepints/Items/BP_PiramidaDown.BP_PiramidaDown_C" (Math|Transform|MakeTransform "0, 0, 0" "0, 0, 0" "1.000000,1.000000,1.000000") "Undefined" "MultiplyWithRoot" 0 0 "0.000000,0.000000,0.000000" false 0)
    (Development|PrintString "Ты решил загадку")
    (else
      (Development|PrintString "Ты разложил не все фигуры"))))

(event EventBeginPlay
  (|CallParentFunction))

(event Collision|EventActorBeginOverlap
  (params (OtherActor :type Actor%20Object%20Reference))
  (|CallParentFunction OtherActor)
  (CallFunction|SummIndex))

(event EventTick
  (params (DeltaSeconds :type Float%20%28single-precision%29))
  (|CallParentFunction DeltaSeconds) ; This node is disabled and will not be called.\nDrag off pins to build functionality.
)

(fn ConstructionScript
  (|CallParentFunction))

(fn CheckIndex)

(fn GetDropItemIndex
  (return 0))

(fn GetPickupItem
  (return false))

(fn IndexSumReq
  (Variables|Default|SetIdexSumReqCurrent (+ (Variables|Default|GetIdexSumReqCurrent) 1)))

(fn FunctionTestovaya
  (return false false false false))