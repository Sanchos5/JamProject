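; BP_Letter is a letter actor among the FamilyPhoto items that glides toward a target position.
; Each Tick eases its root component from its current world location toward the NewPosition variable using VInterpTo, without sweeping.
; MoveLetter and GetButtonGridLocations are empty stubs, and nothing in this Blueprint sets NewPosition.
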(event EventBeginPlay
  (|CallParentFunction))

(event Collision|EventActorBeginOverlap
  (params (OtherActor :type Actor%20Object%20Reference))
  (|CallParentFunction OtherActor) ; This node is disabled and will not be called.\nDrag off pins to build functionality.
)

(event EventTick
  (params (DeltaSeconds :type Float%20%28single-precision%29))
  (bind _defaultsceneroot (Variables|Default|GetDefaultSceneRoot))
  (|CallParentFunction DeltaSeconds)
  (Transformation|SetWorldLocation _defaultsceneroot (Math|Interpolation|VInterpTo (Transformation|GetWorldLocation _defaultsceneroot) (Variables|Default|GetNewPosition) DeltaSeconds 1e+01) false false))

(fn ConstructionScript
  (|CallParentFunction))

(fn GetButtonGridLocations
  (return 0))

(fn MoveLetter
  (params (NewLocation :type Vector :default "0, 0, 0"))
  (return))